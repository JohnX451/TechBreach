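; Showcase level-scripting actor that drives a demo quest flow with HUD messages from "Samuel Gray".
; On BeginPlay it queues an intro message and adds the main escape quest after short delays.
; Two one-shot trigger boxes react to the player: one unlocks the armature-install stage, the other adds a side quest to kill cyborgs.
; The construction script positions both boxes from variables.
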(event `self.ReceiveBeginPlay`
  (`KismetSystemLibrary.Delay` 1.0)
  (`/Game/Blueprints/BP_TechFunctions.Queue Hud Message` "Samuel Gray" "I'm giving you a main quest: escape this level. GLHF." "/Game/Blueprints/Items/Textures/ID/T_ID_Atlas.T_ID_Atlas")
  (`KismetSystemLibrary.Delay` 1.0)
  (`/Game/Blueprints/BP_TechFunctions.AddQuest` "Q_M_Test01"))

(event `self.Box_InstallArmature.OnComponentBeginOverlap`
  (params (OverlappedComponent :type "PrimitiveComponent Object Reference") (OtherActor :type "Actor Object Reference") (OtherComp :type "PrimitiveComponent Object Reference") (OtherBodyIndex :type Integer) (bFromSweep :type Boolean) (SweepResult :type "HitResult Structure (by ref)"))
  (cast `/Game/Blueprints/Player/BP_PlayerCharacter` OtherActor)
  (`/Engine/EditorBlueprintResources/StandardMacros.DoOnce` false
    (:`Completed`
      (`/Game/Blueprints/BP_TechFunctions.Queue Hud Message` "Samuel Gray" "Oh yeah, install the modular servo armature to get through the first door." "/Game/Blueprints/Items/Textures/ID/T_ID_Atlas.T_ID_Atlas")
      (`KismetSystemLibrary.Delay` 1.0)
      (`/Game/Blueprints/BP_TechFunctions.UnlockQuestStage` "Q_M_Test01_S02"))))

(event `self.Box_KillDudes.OnComponentBeginOverlap`
  (params (OverlappedComponent :type "PrimitiveComponent Object Reference") (OtherActor :type "Actor Object Reference") (OtherComp :type "PrimitiveComponent Object Reference") (OtherBodyIndex :type Integer) (bFromSweep :type Boolean) (SweepResult :type "HitResult Structure (by ref)"))
  (cast `/Game/Blueprints/Player/BP_PlayerCharacter` OtherActor)
  (`/Engine/EditorBlueprintResources/StandardMacros.DoOnce` false
    (:`Completed`
      (`/Game/Blueprints/BP_TechFunctions.Queue Hud Message` "Samuel Gray" "Jesus those Cyborgs suck. Kill them." "/Game/Blueprints/Items/Textures/ID/T_ID_Atlas.T_ID_Atlas")
      (`KismetSystemLibrary.Delay` 1.0)
      (`/Game/Blueprints/BP_TechFunctions.AddQuest` "Q_S_Test02"))))

(fn `UserConstructionScript`
  (`SceneComponent.K2_SetRelativeLocation` (`self.Box_InstallArmature`) (`self.Box_Install_Position`) false false)
  (`SceneComponent.K2_SetRelativeLocation` (`self.Box_KillDudes`) (`self.Box_KillDudes_Position`) false false))