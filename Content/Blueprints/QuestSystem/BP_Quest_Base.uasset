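; Base quest actor that tracks objective progress through the stages of one quest.
; It loads stage data from DT_QuestData by QuestID and updates a progress map from the player's objective ID event, pre-crediting installed implants at BeginPlay for one objective type.
; Completed objectives show a HUD notification; finished stages load the next, and the last marks completion, turning in through AC_QuestLog if auto-complete is set.
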(event `self.ReceiveBeginPlay`
  (`self.GetQuestDetails`)
  ;[1 1 1] Bind Event when Quest Objectives are completed
  (bind _asbp_player_character (cast `/Game/Blueprints/Player/BP_PlayerCharacter` (`GameplayStatics.GetPlayerCharacter` 0)))
  (add `/Game/Blueprints/Player/BP_PlayerCharacter.OnObjectiveIDCalled` _asbp_player_character (`|CreateDelegate` :!event `On Objective IDHeard`))
  ;[1 1 1] Get Collect Objectives
  (for _array_element (`.Objectives_8_435DD1A941CA50FD96E644B481F39ADA` (break `/Game/Blueprints/QuestSystem/F_StageDetails` (`self.CurrentStageDetails`)))
    (if (`|EnumEquality` (`.Type_16_C9BA69B34F71B7C5E9B1AD89DB1D6DFB` (break `/Game/Blueprints/QuestSystem/F_ObjectiveDetails` _array_element)) "NewEnumerator3")
      ;[1 1 1] Check how many Items are in the Inventory and Update corresponding Objective Progress
      (bind _asbp_player_character_2 (cast `/Game/Blueprints/Player/BP_PlayerCharacter` (`GameplayStatics.GetPlayerCharacter` 0)))
      ;[1 1 1] Check if a module already is installed and update objective accordingly
      (bind _values (`BlueprintMapLibrary.Map_Values` (`ModulesComponent.ActiveImplants` (`/Game/Blueprints/Player/BP_PlayerCharacter.BP_ModulesComponent` _asbp_player_character_2))))
      (for _array_element_2 _values
        (`self.On Objective IDHeard` (`KismetStringLibrary.Conv_NameToString` (`.Id` (break `ImplantData` _array_element_2)))))))
  (`KismetSystemLibrary.Delay` 1.0)
  ;[1 1 1] Tracks completion
  (bind _return (`self.Are Objectives Complete`))
  (set `self.isCompleted` _return))

(fn `Are Objectives Complete`
  (returns (Return :type Boolean))
  (locals (Local_AllComplete :type Boolean :default true))
  (for _array_element (`.Objectives_8_435DD1A941CA50FD96E644B481F39ADA` (break `/Game/Blueprints/QuestSystem/F_StageDetails` (`self.CurrentStageDetails`)))
    (bind (_objectivename _description _type _objectiveid) (break `/Game/Blueprints/QuestSystem/F_ObjectiveDetails` _array_element))
    (if (not (>= (`BlueprintMapLibrary.Map_Find` (`self.CurrentObjectiveProgress`) _objectiveid) (`.Quantity_15_6770E1EF48594C30D446F3947818828B` (break `/Game/Blueprints/QuestSystem/F_ObjectiveDetails` (`self.GetObjectiveDataByID` _objectiveid)))))
      (bind _output_get (set `local.Local_AllComplete` false))
      (return _output_get)))
  (return (`local.Local_AllComplete`)))

(fn `GetObjectiveDataByID`
  (params (ObjectiveID :type String))
  (returns (`Array Element` :type "/Game/Blueprints/QuestSystem/F_ObjectiveDetails Structure"))
  (for _array_element (`.Objectives_8_435DD1A941CA50FD96E644B481F39ADA` (break `/Game/Blueprints/QuestSystem/F_StageDetails` (`self.CurrentStageDetails`)))
    (if (`KismetStringLibrary.EqualEqual_StrStr` (`.ObjectiveID_9_BEA5C2B047A9B3FC5991D2BEAF3D97B3` (break `/Game/Blueprints/QuestSystem/F_ObjectiveDetails` _array_element)) ObjectiveID)
      (return _array_element))))

(fn `GetQuestDetails`
  ;[1 1 1] Gets Quest State Details
  (bind _returnvalue (`|GetDataTableRow` "/Game/QuestSystem/DT_QuestData.DT_QuestData" (`self.QuestID`))
    (:`then`
      (bind _output_get (set `self.QuestDetails` _returnvalue))
      (bind _output_get_2 (set `self.CurrentStageDetails` (`|GetArrayItem` (`.Stages_13_AA0821FA40E4ABBB49391F8BDB72A14E` (break `/Game/Blueprints/QuestSystem/F_QuestDetails` _output_get)) (`self.CurrentStage`))))
      ;[1 1 1] Set all ObjectiveIDs to 0 when initiating
      (`BlueprintMapLibrary.Map_Clear` (`self.CurrentObjectiveProgress`))
      (for _array_element (`.Objectives_8_435DD1A941CA50FD96E644B481F39ADA` (break `/Game/Blueprints/QuestSystem/F_StageDetails` _output_get_2))
        (`BlueprintMapLibrary.Map_Add` (`self.CurrentObjectiveProgress`) (`.ObjectiveID_9_BEA5C2B047A9B3FC5991D2BEAF3D97B3` (break `/Game/Blueprints/QuestSystem/F_ObjectiveDetails` _array_element)))))))

(fn `IsObjectiveComplete`
  (params (ObjectiveID :type String))
  (bind (_questdetails_questname _questdetails_logdescription _questdetails_trackingdescription _questdetails_ismainquest _questdetails_stages) (break `/Game/Blueprints/QuestSystem/F_QuestDetails` (`self.QuestDetails`)))
  (bind (_questdetails_questname_2 _questdetails_logdescription_2 _questdetails_trackingdescription_2 _questdetails_ismainquest_2 _questdetails_stages_2 _questdetails_autoaccept _questdetails_autocomplete) (break `/Game/Blueprints/QuestSystem/F_QuestDetails` (`self.QuestDetails`)))
  (bind ((`Description_4_BE1EFBD4419A630BBABDF9BCFF5E4877` _description) (`Quantity_15_6770E1EF48594C30D446F3947818828B` _quantity)) (break `/Game/Blueprints/QuestSystem/F_ObjectiveDetails` (`self.GetObjectiveDataByID` ObjectiveID)))
  (if (>= (`BlueprintMapLibrary.Map_Find` (`self.CurrentObjectiveProgress`) (`local.ObjectiveID`)) _quantity)
    ;[1 1 1] Add Notification on HUD
    (bind _returnvalue (`|CreateWidget` "/Game/Blueprints/QuestSystem/UI/WBP_QuestNotification.WBP_QuestNotification_C" null _description))
    (`UserWidget.AddToViewport` _returnvalue 0)
    ;[1 1 1] Tracks completion
    (bind _return (`self.Are Objectives Complete`))
    (if _return
      (bind _result (`/Engine/EditorBlueprintResources/StandardMacros.IncrementInt` (`self.CurrentStage`))
        (:`  `
          (if (`KismetArrayLibrary.Array_IsValidIndex` _questdetails_stages _result)
            (`self.GetQuestDetails`)
            (else
              (set `self.isCompleted` true)
              ;[1 1 1] Auto complete
              (if _questdetails_autocomplete
                (bind _asbp_player_character (cast `/Game/Blueprints/Player/BP_PlayerCharacter` (`GameplayStatics.GetPlayerCharacter` 0)))
                (`/Game/Blueprints/QuestSystem/AC_QuestLog.TurnInQuest` (`self.GetComponentByClass` _asbp_player_character "/Game/Blueprints/QuestSystem/AC_QuestLog.AC_QuestLog_C") (`self.QuestID`))))))))))

(fn `On Objective IDHeard`
  (params (ObjectiveID :type String) (Value :type Integer :default 1))
  (bind (_value _returnvalue) (`BlueprintMapLibrary.Map_Find` (`self.CurrentObjectiveProgress`) (`local.ObjectiveID`)))
  (if (> (`KismetMathLibrary.SignOfInteger` Value) 0)
    ;[1 1 1] Adds to Objective Progress
    (if _returnvalue
      (if (< _value (`.Quantity_15_6770E1EF48594C30D446F3947818828B` (break `/Game/Blueprints/QuestSystem/F_ObjectiveDetails` (`self.GetObjectiveDataByID` (`local.ObjectiveID`)))))
        (`BlueprintMapLibrary.Map_Add` (`self.CurrentObjectiveProgress`) (`local.ObjectiveID`) (+ _value (`local.Value`)))
        (`self.IsObjectiveComplete` (`local.ObjectiveID`))
        (`self.OnObjectiveHeard`)
        (return))
      (else
        (return)))
    (else
      ;[1 1 1] Diminishing Objective Progress
      (`BlueprintMapLibrary.Map_Add` (`self.CurrentObjectiveProgress`) (`local.ObjectiveID`) (+ (`BlueprintMapLibrary.Map_Find` (`self.CurrentObjectiveProgress`) (`local.ObjectiveID`)) (`local.Value`)))
      (return))))

(fn `UserConstructionScript`)