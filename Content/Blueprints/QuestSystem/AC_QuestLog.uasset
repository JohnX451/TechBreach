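; AC_QuestLog is a quest log component that records active and completed quests by ID and offers queries on both.
; Adding a quest spawns a BP_Quest_Base actor to represent it, while tracking one lazily creates or updates a single WBP_Tracker widget.
; Turn-in runs CompleteQuest, which moves the ID to completed, flags the actor, fires OnQuestCompleted and unlists the actor without destroying it.
; The completed query reports turned-in whenever no quest actor is found.
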(fn `AddNewQuest`
  (params (QuestID :type Name))
  (`KismetArrayLibrary.Array_AddUnique` (`self.CurrentActiveQuests`) QuestID)
  (bind _returnvalue (`|SpawnActorFromClass` "/Game/Blueprints/QuestSystem/BP_Quest_Base.BP_Quest_Base_C" (`KismetMathLibrary.MakeTransform` (0.0 0.0 0.0)) "Undefined" "MultiplyWithRoot" null QuestID null))
  (`KismetArrayLibrary.Array_Add` (`self.CurrentQuests`) _returnvalue))

(fn `CompleteQuest`
  (params (QuestID :type Name))
  ;[1 1 1] Removes completed Quests from current ones
  (`KismetArrayLibrary.Array_AddUnique` (`self.CompletedQuests`) QuestID)
  (`KismetArrayLibrary.Array_RemoveItem` (`self.CurrentActiveQuests`) QuestID)
  (bind _array_element (`self.GetQuestActor` QuestID))
  (set `/Game/Blueprints/QuestSystem/BP_Quest_Base.isTurnedIn` true _array_element)
  (`self.OnQuestCompleted` _array_element)
  ;[1 1 1] Remove completed Quest from the Log
  (`KismetArrayLibrary.Array_RemoveItem` (`self.CurrentQuests`) _array_element))

(fn `GetQuestActor`
  (params (QuestID :type Name))
  (returns (`Array Element` :type "/Game/Blueprints/QuestSystem/BP_Quest_Base Object Reference"))
  (for _array_element (`self.CurrentQuests`)
    (if (== (`/Game/Blueprints/QuestSystem/BP_Quest_Base.QuestID` _array_element) QuestID)
      (return _array_element))))

(fn `QuerryActiveQuest`
  (params (QuestID :type Name))
  (returns (ReturnValue :type Boolean))
  (return (`KismetArrayLibrary.Array_Contains` (`self.CurrentActiveQuests`) QuestID)))

(fn `QuerryCompletedQuest`
  (params (QuestID :type Name))
  (returns (ReturnValue :type Boolean) (turnedIn :type Boolean))
  (bind _returnvalue (`KismetArrayLibrary.Array_Contains` (`self.CompletedQuests`) QuestID))
  (bind _array_element (`self.GetQuestActor` QuestID))
  (`/Engine/EditorBlueprintResources/StandardMacros.IsValid` _array_element
    (:`Is Valid`
      (return _returnvalue (`/Game/Blueprints/QuestSystem/BP_Quest_Base.isTurnedIn` _array_element)))
    (:`Is Not Valid`
      (return _returnvalue true))))

(fn `TrackQuest`
  (params (QuestActor :type "/Game/Blueprints/QuestSystem/BP_Quest_Base Object Reference"))
  (bind _tracker (`self.Tracker`)
    (:`then`
      (`/Game/Blueprints/QuestSystem/UI/WBP_Tracker.Update` _tracker QuestActor))
    (:`else`
      (bind _returnvalue (`|CreateWidget` "/Game/Blueprints/QuestSystem/UI/WBP_Tracker.WBP_Tracker_C" null QuestActor))
      (bind _output_get (set `self.Tracker` _returnvalue))
      (`UserWidget.AddToViewport` _output_get -1))))

(fn `TurnInQuest`
  (params (QuestID :type Name))
  (`self.CompleteQuest` QuestID))