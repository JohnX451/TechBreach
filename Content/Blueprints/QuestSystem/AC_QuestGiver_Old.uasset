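; Legacy quest giver component that, on interaction, is meant to offer a data-table quest or show its rewards.
; DisplayQuest and DisplayRewards each look up the quest row and add a widget to the viewport, with rewards hardcoded to the Level01 table.
; InteractWith is unfinished: quest-log and auto-accept conditions are constants, so it always reaches an empty auto-accept branch.
; The completed-quest rewards check is disconnected.
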(fn `DisplayQuest`
  (bind (_questdata_datatable _questdata_rowname) (break `DataTableRowHandle` (`self.QuestData`)))
  (bind _returnvalue (`|GetDataTableRow` _questdata_datatable _questdata_rowname)
    (:`then`
      (bind _returnvalue_2 (`|CreateWidget` "/Game/Blueprints/QuestSystem/UI/WBP_QuestGiver.WBP_QuestGiver_C" null _returnvalue _questdata_rowname))
      (`UserWidget.AddToViewport` _returnvalue_2 0))))

(fn `DisplayRewards`
  (bind (_questdata_datatable _questdata_rowname) (break `DataTableRowHandle` (`self.QuestData`)))
  (bind _returnvalue (`|GetDataTableRow` "/Game/DataTables/DT_QuestData_Level01.DT_QuestData_Level01" _questdata_rowname)
    (:`then`
      (bind _returnvalue_2 (`|CreateWidget` "/Game/Blueprints/QuestSystem/UI/WBP_QuestRewards.WBP_QuestRewards_C" null _returnvalue _questdata_rowname))
      (`UserWidget.AddToViewport` _returnvalue_2 0))))

(fn `InteractWith`
  (returns (ObjectiveID :type String))
  (bind (_questdata_datatable _questdata_rowname) (break `DataTableRowHandle` (`self.QuestData`)))
  ;[1 1 1] Check if Quest already in Quest Log or completed
  (bind _asbp_player_character (cast `/Game/Blueprints/Player/BP_PlayerCharacter` (`GameplayStatics.GetPlayerCharacter` 0)))
  (if (and (not false) (not false))
    ;[1 1 1] Check for auto accept
    (bind _returnvalue (`|GetDataTableRow` "/Game/DataTables/DT_QuestData_Level01.DT_QuestData_Level01" _questdata_rowname)
      (:`then`
        (if true
          ;[1 1 1] Auto Accept
          (`/Engine/EditorBlueprintResources/StandardMacros.IsValid` (`Actor.GetComponentByClass` (`GameplayStatics.GetPlayerCharacter` 0) "/Game/Blueprints/QuestSystem/BP_QuestLogComponent.BP_QuestLogComponent_C"))
          (else
            ;[1 1 1] Display Quest
            (`self.DisplayQuest`)
            (return (`KismetSystemLibrary.GetDisplayName` (`self.GetOwner`)))))))
    (else
      ;[1 1 1] Check for completed Quest
      (bind _asbp_player_character_2 (cast `/Game/Blueprints/Player/BP_PlayerCharacter` (`GameplayStatics.GetPlayerCharacter` 0))))))