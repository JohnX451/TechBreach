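; AC_QuestGiver is an actor component that offers a data-table quest to the player and presents its rewards on completion.
; InteractWith checks the player's quest log, then either auto-accepts a new quest or opens WBP_QuestGiver.
; For a completed quest not yet turned in, it opens WBP_QuestRewards.
; DisplayQuest reads the table from the QuestData row handle, while the other lookups hard-code DT_QuestData.
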(fn `DisplayQuest`
  (bind (_questdata_datatable _questdata_rowname) (break `DataTableRowHandle` (`self.QuestData`)))
  (bind _returnvalue (`|GetDataTableRow` _questdata_datatable _questdata_rowname)
    (:`then`
      (bind _returnvalue_2 (`|CreateWidget` "/Game/Blueprints/QuestSystem/UI/WBP_QuestGiver.WBP_QuestGiver_C" null _returnvalue _questdata_rowname))
      (`UserWidget.AddToViewport` _returnvalue_2 0))))

(fn `DisplayRewards`
  (bind (_questdata_datatable _questdata_rowname) (break `DataTableRowHandle` (`self.QuestData`)))
  (bind _returnvalue (`|GetDataTableRow` "/Game/QuestSystem/DT_QuestData.DT_QuestData" _questdata_rowname)
    (:`then`
      (bind _returnvalue_2 (`|CreateWidget` "/Game/Blueprints/QuestSystem/UI/WBP_QuestRewards.WBP_QuestRewards_C" null _returnvalue _questdata_rowname))
      (`UserWidget.AddToViewport` _returnvalue_2 0))))

(fn `InteractWith`
  (returns (ObjectiveID :type String))
  (bind (_questdata_datatable _questdata_rowname) (break `DataTableRowHandle` (`self.QuestData`)))
  (bind (_questdata_datatable_2 _questdata_rowname_2) (break `DataTableRowHandle` (`self.QuestData`)))
  (bind (_questdata_datatable_3 _questdata_rowname_3) (break `DataTableRowHandle` (`self.QuestData`)))
  (bind (_questdata_datatable_4 _questdata_rowname_4) (break `DataTableRowHandle` (`self.QuestData`)))
  (bind _returnvalue (`Actor.GetComponentByClass` (`GameplayStatics.GetPlayerCharacter` 0) "/Game/Blueprints/QuestSystem/AC_QuestLog.AC_QuestLog_C"))
  ;[1 1 1] Check if Quest already in Quest Log or completed
  (bind _asbp_player_character (cast `/Game/Blueprints/Player/BP_PlayerCharacter` (`GameplayStatics.GetPlayerCharacter` 0)))
  (bind _ac_questlog (`/Game/Blueprints/Player/BP_PlayerCharacter.AC_QuestLog` _asbp_player_character))
  (if (and (not (`/Game/Blueprints/QuestSystem/AC_QuestLog.QuerryActiveQuest` _ac_questlog _questdata_rowname_2)) (not (`/Game/Blueprints/QuestSystem/AC_QuestLog.QuerryCompletedQuest` _ac_questlog _questdata_rowname_2)))
    ;[1 1 1] Check for auto accept
    (bind _returnvalue_2 (`|GetDataTableRow` "/Game/QuestSystem/DT_QuestData.DT_QuestData" _questdata_rowname_4)
      (:`then`
        (if (`.AutoAccept_15_3A6CC9C140781BBA486BCEBBCB0D0EB8` (break `/Game/Blueprints/QuestSystem/F_QuestDetails` _returnvalue_2))
          ;[1 1 1] Auto Accept
          (`/Engine/EditorBlueprintResources/StandardMacros.IsValid` _returnvalue
            (:`Is Valid`
              (`/Game/Blueprints/QuestSystem/AC_QuestLog.AddNewQuest` _returnvalue _questdata_rowname_3)))
          (else
            ;[1 1 1] Display Quest
            (`self.DisplayQuest`)))
        (return (`KismetSystemLibrary.GetDisplayName` (`self.GetOwner`)))))
    (else
      ;[1 1 1] Check for completed Quest
      (bind _asbp_player_character_2 (cast `/Game/Blueprints/Player/BP_PlayerCharacter` (`GameplayStatics.GetPlayerCharacter` 0)))
      (bind _array_element (`/Game/Blueprints/QuestSystem/AC_QuestLog.GetQuestActor` (`/Game/Blueprints/Player/BP_PlayerCharacter.AC_QuestLog` _asbp_player_character_2) _questdata_rowname))
      (if (and (`/Game/Blueprints/QuestSystem/BP_Quest_Base.isCompleted` _array_element) (not (`/Game/Blueprints/QuestSystem/BP_Quest_Base.isTurnedIn` _array_element)))
        (`self.DisplayRewards`)
        (return (`KismetSystemLibrary.GetDisplayName` (`self.GetOwner`)))))))