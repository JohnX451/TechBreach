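; Older quest base Blueprint that tracks one quest's staged objectives and completion.
; On BeginPlay it loads the QuestID row from DT_QuestData_Level01 and resets the current stage's progress map.
; OnObjectiveIDHeard adjusts progress; increases can show a HUD notification, advance stages or complete the quest.
; Objective field references are blank, completion tests only check progress >= 0, and inventory and implant pre-checks are disconnected.
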(event `self.ReceiveBeginPlay`
  (`self.GetQuestDetails`)
  ;[1 1 1] Bind Event when Quest Objectives are completed
  (cast `/Game/Blueprints/Player/BP_PlayerCharacter` (`GameplayStatics.GetPlayerCharacter` 0)))

(fn `Are Objectives Complete`
  (returns (Return :type Boolean))
  (locals (Local_AllComplete :type Boolean :default true))
  (for _ (`.Objectives_8_435DD1A941CA50FD96E644B481F39ADA` (break `/Game/Blueprints/QuestSystem/F_StageDetails` (`self.CurrentStageDetails`)))
    (if (not (>= (`BlueprintMapLibrary.Map_Find` (`self.CurrentObjectiveProgress`)) 0))
      (bind _output_get (set `local.Local_AllComplete` false))
      (return _output_get)))
  (return (`local.Local_AllComplete`)))

(fn `GetObjectiveDataByID`
  (params (ObjectiveID :type String))
  (returns (`Array Element` :type "/Game/Blueprints/QuestSystem/F_ObjectiveDetails Structure"))
  (for _array_element (`.Objectives_8_435DD1A941CA50FD96E644B481F39ADA` (break `/Game/Blueprints/QuestSystem/F_StageDetails` (`self.CurrentStageDetails`)))
    (if (`KismetStringLibrary.EqualEqual_StrStr` "" ObjectiveID)
      (return _array_element))))

(fn `GetQuestDetails`
  ;[1 1 1] Gets Quest State Details
  (bind _returnvalue (`|GetDataTableRow` "/Game/DataTables/DT_QuestData_Level01.DT_QuestData_Level01" (`self.QuestID`))
    (:`then`
      (bind _output_get (set `self.QuestDetails` _returnvalue))
      (bind _output_get_2 (set `self.CurrentStageDetails` (`|GetArrayItem` (`.Stages_13_AA0821FA40E4ABBB49391F8BDB72A14E` (break `/Game/Blueprints/QuestSystem/F_QuestDetails` _output_get)) (`self.CurrentStage`))))
      ;[1 1 1] Set all ObjectiveIDs to 0 when initiating
      (`BlueprintMapLibrary.Map_Clear` (`self.CurrentObjectiveProgress`))
      (for _ (`.Objectives_8_435DD1A941CA50FD96E644B481F39ADA` (break `/Game/Blueprints/QuestSystem/F_StageDetails` _output_get_2))
        (`BlueprintMapLibrary.Map_Add` (`self.CurrentObjectiveProgress`))))))

(fn `IsObjectiveComplete`
  (params (ObjectiveID :type String))
  (bind (_questdetails_questid _questdetails_questname _questdetails_logdescription _questdetails_ismainquest _questdetails_stages) (break `/Game/Blueprints/QuestSystem/F_QuestDetails` (`self.QuestDetails`)))
  (if (>= (`BlueprintMapLibrary.Map_Find` (`self.CurrentObjectiveProgress`) (`local.ObjectiveID`)) 0)
    ;[1 1 1] Add Notification on HUD
    (bind _returnvalue (`|CreateWidget` "/Game/Blueprints/QuestSystem/UI/WBP_QuestNotification.WBP_QuestNotification_C"))
    (`UserWidget.AddToViewport` _returnvalue 0)
    ;[1 1 1] Tracks completion
    (bind _return (`self.Are Objectives Complete`))
    (if _return
      (bind _result (`/Engine/EditorBlueprintResources/StandardMacros.IncrementInt` (`self.CurrentStage`))
        (:`  `
          (if (`KismetArrayLibrary.Array_IsValidIndex` _questdetails_stages _result)
            (`self.GetQuestDetails`)
            (else
              (set `self.isCompleted` true)
              ;[1 1 1] Auto complete
              (if true
                (cast `/Game/Blueprints/Player/BP_PlayerCharacter` (`GameplayStatics.GetPlayerCharacter` 0))))))))))

(fn `On Objective IDHeard`
  (params (ObjectiveID :type String) (Value :type Integer :default 1))
  (bind (_value _returnvalue) (`BlueprintMapLibrary.Map_Find` (`self.CurrentObjectiveProgress`) (`local.ObjectiveID`)))
  (if (> (`KismetMathLibrary.SignOfInteger` Value) 0)
    ;[1 1 1] Adds to Objective Progress
    (if _returnvalue
      (if true
        (`BlueprintMapLibrary.Map_Add` (`self.CurrentObjectiveProgress`) (`local.ObjectiveID`) (+ _value (`local.Value`)))
        (`self.IsObjectiveComplete` (`local.ObjectiveID`))
        (`self.OnObjectiveHeard`)
        (return))
      (else
        (return)))
    (else
      ;[1 1 1] Diminishing Objective Progress
      (`BlueprintMapLibrary.Map_Add` (`self.CurrentObjectiveProgress`) (`local.ObjectiveID`) (+ (`BlueprintMapLibrary.Map_Find` (`self.CurrentObjectiveProgress`) (`local.ObjectiveID`)) (`local.Value`)))
      (return))))

(fn `UserConstructionScript`)