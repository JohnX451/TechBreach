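; Actor component that lets its owning actor drive the quest system when interacted with.
; It stores an interaction type and ID, and QuestInteraction uses them to add a quest, unlock a quest stage or complete an objective, skipping a None ID.
; UpdateDataForNextInteraction overwrites both values, so the same actor can trigger a different quest action next time.
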(event `QuestInteraction`
  (bind _interactionid (`self.InteractionId`))
  (if (!= (`self.InteractionId`) "None")
    (switch `/Game/Blueprints/QuestSystem/E_QuestInteractionType` (`self.InteractionType`)
      (:`NewEnumerator0`
        (`/Game/Blueprints/BP_TechFunctions.AddQuest` _interactionid))
      (:`NewEnumerator1`
        (`/Game/Blueprints/BP_TechFunctions.UnlockQuestStage` _interactionid))
      (:`NewEnumerator2`
        (`/Game/Blueprints/BP_TechFunctions.CompleteObjective` _interactionid)))))

(event `UpdateDataForNextInteraction`
  (params (InteractionType :type "/Game/Blueprints/QuestSystem/E_QuestInteractionType Enum" :default "NewEnumerator0") (InteractionId :type Name))
  (set `self.InteractionType` InteractionType)
  (set `self.InteractionId` InteractionId))