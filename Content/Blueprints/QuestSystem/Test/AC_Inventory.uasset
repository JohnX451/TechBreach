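; AC_Inventory is an inventory component in the quest system's test folder that tracks item quantities.
; AddToInventory adds the given quantity to the item's existing count in the Content map, and QuerryInventory returns that count.
; A player notification with the item name is unfinished: AddToInventory casts to BP_PlayerCharacter but does nothing with the result.
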(fn `AddToInventory`
  (params (Item :type Name) (Quantity :type Integer))
  ;[1 1 1] Add Item to Inventory
  (`BlueprintMapLibrary.Map_Add` (`self.Content`) Item (+ Quantity (`BlueprintMapLibrary.Map_Find` (`self.Content`) Item)))
  ;[1 1 1] Notify Player with Item Name
  (cast `/Game/Blueprints/Player/BP_PlayerCharacter` (`GameplayStatics.GetPlayerCharacter` 0)))

(fn `QuerryInventory`
  (params (Item :type Name))
  (returns (Value :type Integer))
  (return (`BlueprintMapLibrary.Map_Find` (`self.Content`) Item)))