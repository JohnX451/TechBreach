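; Quest log component that loads the level's quests from a data table on BeginPlay, after a short delay so level scripting can override the table.
; AddQuest and UnlockQuestStage reveal quests and stages by ID, writing rebuilt structs back through SetQuestData.
; CompleteObjective rolls completion up from objectives to stages to quests.
; These changes play UI sounds and broadcast the visible, unfinished main quest and its open stages to the tracker.
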(event `self.ReceiveBeginPlay`
  ;[1 1 1 1 12] wait, so level scripting can ovveride data table if necessary
  (`KismetSystemLibrary.Delay` 0.2)
  ;[1 1 1] Set up quest structures for the current level
  (bind _outrownames (`DataTableFunctionLibrary.GetDataTableRowNames` (`self.LevelQuestData`)))
  (for _index (range (`KismetArrayLibrary.Array_Length` _outrownames))
    (bind _returnvalue (`|GetDataTableRow` (`self.LevelQuestData`) (`|GetArrayItem` _outrownames _index))
      (:`then`
        (`KismetArrayLibrary.Array_Add` (`self.Quests`) _returnvalue)))))

(fn `AddQuest`
  (params (QuestId :type Name))
  (bind (_bisactive _biscompleted) (`self.IsQuestActiveOrCompleted` QuestId))
  (if (not _bisactive)
    (bind _quest (`self.GetQuestById` QuestId))
    (bind (_questid _questname _logdescription _ismainquest _stages) (break `/Game/Blueprints/QuestSystem/F_QuestDetails` _quest))
    (`self.SetQuestData` (make `/Game/Blueprints/QuestSystem/F_QuestDetails` _questid _questname _logdescription _ismainquest _stages _biscompleted true))
    (`self.UpdateTracker`)
    (`GameplayStatics.PlaySound2D` "/Game/Audio/UI/Waves/S_UI_Quest_New.S_UI_Quest_New" 1.0 1.0 0.0 null null)))

(fn `CheckForCompletion`
  (params (QuestId :type Name))
  (locals (CompletedStages :type Integer))
  (bind _quest (`self.GetQuestById` QuestId))
  (for _array_element (`.Stages_13_AA0821FA40E4ABBB49391F8BDB72A14E` (break `/Game/Blueprints/QuestSystem/F_QuestDetails` _quest))
    (if (`.IsCompleted_10_15F2143942C8E6DE041044AA1CE99340` (break `/Game/Blueprints/QuestSystem/F_StageDetails` _array_element))
      (`/Engine/EditorBlueprintResources/StandardMacros.IncrementInt` (`local.CompletedStages`))))
  (bind _returnvalue (== (`KismetArrayLibrary.Array_Length` (`.Stages_13_AA0821FA40E4ABBB49391F8BDB72A14E` (break `/Game/Blueprints/QuestSystem/F_QuestDetails` _quest))) (`local.CompletedStages`)))
  (`self.SetQuestData` (make `/Game/Blueprints/QuestSystem/F_QuestDetails` (break `/Game/Blueprints/QuestSystem/F_QuestDetails` _quest) (`.QuestName_2_66C12911419EF45B09551FB52C56AEC5` (break `/Game/Blueprints/QuestSystem/F_QuestDetails` _quest)) (`.LogDescription_4_BC32F9D84DA3621CCB888F94B6535147` (break `/Game/Blueprints/QuestSystem/F_QuestDetails` _quest)) (`.IsMainQuest_24_7FB9AC0941515A897C46E3A032916005` (break `/Game/Blueprints/QuestSystem/F_QuestDetails` _quest)) (`.Stages_13_AA0821FA40E4ABBB49391F8BDB72A14E` (break `/Game/Blueprints/QuestSystem/F_QuestDetails` _quest)) _returnvalue (`.IsVisible_27_F4DB0AF6405BF04FA5CC0A8BA573F138` (break `/Game/Blueprints/QuestSystem/F_QuestDetails` _quest))))
  (if _returnvalue
    (`GameplayStatics.PlaySound2D` "/Game/Audio/UI/Waves/S_UI_Quest_Complete.S_UI_Quest_Complete" 1.0 1.0 0.0 null null))
  (return))

(fn `CompleteObjective`
  (params (ObjectiveId :type Name))
  (locals (TempStages :type "Array of /Game/Blueprints/QuestSystem/F_StageDetails Structure") (TempObjectives :type "Array of /Game/Blueprints/QuestSystem/F_ObjectiveDetails Structure") (CompletedObjectives :type Integer))
  (bind _objectiveid (`local.ObjectiveId`))
  (for _array_element (`self.Quests`)
    (bind _output_get (set `local.TempStages` (`.Stages_13_AA0821FA40E4ABBB49391F8BDB72A14E` (break `/Game/Blueprints/QuestSystem/F_QuestDetails` _array_element))))
    (for (_array_element_2 _array_index) _output_get
      (bind _output_get_2 (set `local.TempObjectives` (`.Objectives_8_435DD1A941CA50FD96E644B481F39ADA` (break `/Game/Blueprints/QuestSystem/F_StageDetails` _array_element_2))))
      (set `local.CompletedObjectives` 0)
      (for (_array_element_3 _array_index_2) _output_get_2
        (`|ExecutionSequence`
          (:`then_0`
            (bind _returnvalue (== _objectiveid (break `/Game/Blueprints/QuestSystem/F_ObjectiveDetails` _array_element_3)))
            (if _returnvalue
              (`KismetArrayLibrary.Array_Set` (`local.TempObjectives`) _array_index_2 (make `/Game/Blueprints/QuestSystem/F_ObjectiveDetails` _objectiveid true))))
          (:`then_1`
            (if (or _returnvalue (`.IsCompleted_22_7877492D43881A7F70613BB0F53702EE` (break `/Game/Blueprints/QuestSystem/F_ObjectiveDetails` _array_element_3)))
              (`/Engine/EditorBlueprintResources/StandardMacros.IncrementInt` (`local.CompletedObjectives`))))))
      (`KismetArrayLibrary.Array_Set` (`local.TempStages`) _array_index (make `/Game/Blueprints/QuestSystem/F_StageDetails` (break `/Game/Blueprints/QuestSystem/F_StageDetails` _array_element_2) (`.StageName_2_039C471A4D66E2079585E4B14F2FBF6F` (break `/Game/Blueprints/QuestSystem/F_StageDetails` _array_element_2)) (`.Description_4_AA3E44B74A5B933248240280D0510D84` (break `/Game/Blueprints/QuestSystem/F_StageDetails` _array_element_2)) (`local.TempObjectives`) (select `bool` (== (`local.CompletedObjectives`) (`KismetArrayLibrary.Array_Length` (`local.TempObjectives`))) :`false` (`.IsCompleted_10_15F2143942C8E6DE041044AA1CE99340` (break `/Game/Blueprints/QuestSystem/F_StageDetails` _array_element_2)) :`true` true) (`.IsVisible_17_A63063E243C5AC8F26C9CC8E89E2A2C1` (break `/Game/Blueprints/QuestSystem/F_StageDetails` _array_element_2)))))
    (`self.SetQuestData` (make `/Game/Blueprints/QuestSystem/F_QuestDetails` (break `/Game/Blueprints/QuestSystem/F_QuestDetails` _array_element) (`.QuestName_2_66C12911419EF45B09551FB52C56AEC5` (break `/Game/Blueprints/QuestSystem/F_QuestDetails` _array_element)) (`.LogDescription_4_BC32F9D84DA3621CCB888F94B6535147` (break `/Game/Blueprints/QuestSystem/F_QuestDetails` _array_element)) (`.IsMainQuest_24_7FB9AC0941515A897C46E3A032916005` (break `/Game/Blueprints/QuestSystem/F_QuestDetails` _array_element)) (`local.TempStages`) (`.IsCompleted_25_29D2240749EEDE9A83DBFEADEBBCE2DE` (break `/Game/Blueprints/QuestSystem/F_QuestDetails` _array_element)) (`.IsVisible_27_F4DB0AF6405BF04FA5CC0A8BA573F138` (break `/Game/Blueprints/QuestSystem/F_QuestDetails` _array_element))))
    (`self.CheckForCompletion` (break `/Game/Blueprints/QuestSystem/F_QuestDetails` _array_element)))
  (`self.UpdateTracker`))

(fn `GetQuestById`
  (params (QuestId :type Name))
  (returns (Quest :type "/Game/Blueprints/QuestSystem/F_QuestDetails Structure") (bQuestFound :type Boolean))
  (for _array_element (`self.Quests`)
    (if (== (`local.QuestId`) (`.QuestId_30_87A304E44F4955DF43557BB1F5FAC894` (break `/Game/Blueprints/QuestSystem/F_QuestDetails` _array_element)))
      (return _array_element true)))
  (return (struct) false))

(fn `GetVisibleAndCompletedQuests`
  (returns (Quests :type "Array of /Game/Blueprints/QuestSystem/F_QuestDetails Structure"))
  (locals (TempQuests :type "Array of /Game/Blueprints/QuestSystem/F_QuestDetails Structure"))
  (for _array_element (`self.Quests`)
    (bind (_questid _questname _logdescription _ismainquest _stages _iscompleted _isvisible) (break `/Game/Blueprints/QuestSystem/F_QuestDetails` _array_element))
    (if (or _iscompleted _isvisible)
      (`KismetArrayLibrary.Array_Add` (`local.TempQuests`) _array_element)))
  (return (`local.TempQuests`)))

(fn `IsQuestActiveOrCompleted`
  (params (QuestId :type Name))
  (returns (bIsActive :type Boolean) (bIsCompleted :type Boolean))
  (bind (_quest _bquestfound) (`self.GetQuestById` QuestId))
  (if _bquestfound
    (bind (_questid _questname _logdescription _ismainquest _stages _iscompleted _isvisible) (break `/Game/Blueprints/QuestSystem/F_QuestDetails` _quest))
    (return _isvisible _iscompleted)
    (else
      (return false false))))

(fn `SetQuestData`
  (params (NewData :type "/Game/Blueprints/QuestSystem/F_QuestDetails Structure"))
  (locals (FoundQuestId :type Integer))
  (bind (_newdata_questid _newdata_questname _newdata_logdescription _newdata_ismainquest _newdata_stages _newdata_iscompleted _newdata_isvisible) (break `/Game/Blueprints/QuestSystem/F_QuestDetails` (`local.NewData`)))
  (for (_array_element _array_index) (`self.Quests`)
    (if (== (`.QuestId_30_87A304E44F4955DF43557BB1F5FAC894` (break `/Game/Blueprints/QuestSystem/F_QuestDetails` _array_element)) _newdata_questid)
      (`KismetArrayLibrary.Array_Set` (`self.Quests`) _array_index (make `/Game/Blueprints/QuestSystem/F_QuestDetails` _newdata_questid _newdata_questname _newdata_logdescription _newdata_ismainquest _newdata_stages _newdata_iscompleted _newdata_isvisible)))))

(fn `UnlockQuestStage`
  (params (StageId :type Name))
  (locals (TempStages :type "Array of /Game/Blueprints/QuestSystem/F_StageDetails Structure"))
  (for _array_element (`self.Quests`)
    (set `local.TempStages` (`.Stages_13_AA0821FA40E4ABBB49391F8BDB72A14E` (break `/Game/Blueprints/QuestSystem/F_QuestDetails` _array_element)))
    (for (_array_element_2 _array_index) (`.Stages_13_AA0821FA40E4ABBB49391F8BDB72A14E` (break `/Game/Blueprints/QuestSystem/F_QuestDetails` _array_element))
      (if (== (`local.StageId`) (break `/Game/Blueprints/QuestSystem/F_StageDetails` _array_element_2))
        (`KismetArrayLibrary.Array_Set` (`local.TempStages`) _array_index (make `/Game/Blueprints/QuestSystem/F_StageDetails` (break `/Game/Blueprints/QuestSystem/F_StageDetails` _array_element_2) (`.StageName_2_039C471A4D66E2079585E4B14F2FBF6F` (break `/Game/Blueprints/QuestSystem/F_StageDetails` _array_element_2)) (`.Description_4_AA3E44B74A5B933248240280D0510D84` (break `/Game/Blueprints/QuestSystem/F_StageDetails` _array_element_2)) (`.Objectives_8_435DD1A941CA50FD96E644B481F39ADA` (break `/Game/Blueprints/QuestSystem/F_StageDetails` _array_element_2)) (`.IsCompleted_10_15F2143942C8E6DE041044AA1CE99340` (break `/Game/Blueprints/QuestSystem/F_StageDetails` _array_element_2)) true))
        (`self.SetQuestData` (make `/Game/Blueprints/QuestSystem/F_QuestDetails` (break `/Game/Blueprints/QuestSystem/F_QuestDetails` _array_element) (`.QuestName_2_66C12911419EF45B09551FB52C56AEC5` (break `/Game/Blueprints/QuestSystem/F_QuestDetails` _array_element)) (`.LogDescription_4_BC32F9D84DA3621CCB888F94B6535147` (break `/Game/Blueprints/QuestSystem/F_QuestDetails` _array_element)) (`.IsMainQuest_24_7FB9AC0941515A897C46E3A032916005` (break `/Game/Blueprints/QuestSystem/F_QuestDetails` _array_element)) (`local.TempStages`) (`.IsCompleted_25_29D2240749EEDE9A83DBFEADEBBCE2DE` (break `/Game/Blueprints/QuestSystem/F_QuestDetails` _array_element)) true))
        (`self.UpdateTracker`)
        (`GameplayStatics.PlaySound2D` "/Game/Audio/UI/Waves/S_UI_Quest_New.S_UI_Quest_New" 1.0 1.0 0.0 null null)
        (return)))))

(fn `UpdateTracker`
  (locals (TempActiveTitle :type Text) (TempActiveStages :type "Array of Text"))
  (for _array_element (`self.Quests`)
    (bind (_questid _questname _logdescription _ismainquest _stages _iscompleted _isvisible) (break `/Game/Blueprints/QuestSystem/F_QuestDetails` _array_element))
    (if (and _ismainquest (not _iscompleted) _isvisible)
      (set `local.TempActiveTitle` _questname)
      (for _array_element_2 _stages
        (bind (_stageid _stagename _description _objectives _iscompleted_2 _isvisible_2) (break `/Game/Blueprints/QuestSystem/F_StageDetails` _array_element_2))
        (if (and (not _iscompleted_2) _isvisible_2)
          (`KismetArrayLibrary.Array_Add` (`local.TempActiveStages`) _stagename)))))
  (`self.QuestTrackerUpdated` (`local.TempActiveTitle`) (`local.TempActiveStages`)))