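; Hit effects component that provides impact feedback on blood or metal surfaces and can leave blood pools on the floor.
; SpawnImpactEffect spawns a normal-aligned Niagara system by surface type, setting its spawn multiplier before activation, then optionally plays a matching sound with weakspot variants.
; SpawnLiquidPoolOnFloor traces a short distance down against static world geometry and spawns a BP_BloodPool with random yaw, size and growth time.
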(fn `Spawn Impact Effect`
  (params (SurfaceType :type Integer) (HitDamage :type "Float (double-precision)") (bHitWeakspot :type Boolean) (HitLocation :type "Vector Structure") (HitNormal :type "Vector Structure"))
  (locals (EffectCount :type Integer :default 10) (EffectScale :type "Vector Structure" :default (1.0 1.0 1.0)) (HitSFX :type "SoundBase Object Reference") (bPlayImpactSound :type Boolean :default true))
  (bind _surfacetype (`local.SurfaceType`))
  (`|ExecutionSequence`
    (:`then_0`
      (bind _returnvalue (`NiagaraFunctionLibrary.SpawnSystemAtLocation` (select `int` (`local.SurfaceType`) :`0` "/Game/ThirdParty/BallisticsVFX/Particles/Impacts/DynamicImpacts/TechBreach/NS_Impact_Blood.NS_Impact_Blood" :`1` "/Game/ThirdParty/BallisticsVFX/Particles/Impacts/DynamicImpacts/TechBreach/NS_Impact_Metal.NS_Impact_Metal" :!type "NiagaraSystem Object Reference") (`local.HitLocation`) (`KismetMathLibrary.MakeRotFromZ` (`local.HitNormal`)) (`local.EffectScale`) true false))
      (`NiagaraComponent.SetVariableInt` _returnvalue "SpawnMultiplierPercentage" (`local.EffectCount`))
      (`self.Activate` _returnvalue true))
    (:`then_1`
      (if (`local.bPlayImpactSound`)
        (if (`local.bHitWeakspot`)
          (set `local.HitSFX` (select `int` _surfacetype :`0` "/Game/Audio/Weapons/Impacts/MS_Hit_Flesh_Weakspot.MS_Hit_Flesh_Weakspot" :`1` "/Game/Audio/Weapons/Impacts/MS_Hit_Armor_Weakspot.MS_Hit_Armor_Weakspot" :!type "SoundBase Object Reference"))
          (else
            (set `local.HitSFX` (select `int` _surfacetype :`0` "/Game/Audio/Weapons/Impacts/MS_Hit_Flesh.MS_Hit_Flesh" :`1` "/Game/Audio/Weapons/Impacts/MS_Hit_Armor.MS_Hit_Armor" :!type "SoundBase Object Reference"))))
        (`GameplayStatics.PlaySoundAtLocation` (`local.HitSFX`) (`local.HitLocation`) (struct) 1.0 1.0 0.0 null null null null)))))

(fn `SpawnLiquidPoolOnFloor`
  (params (TraceLocation :type "Vector Structure"))
  (bind (_outhit _returnvalue) (`KismetSystemLibrary.LineTraceSingleForObjects` TraceLocation (- TraceLocation (0.0 0.0 100.0)) (`|MakeArray` "ObjectTypeQuery1" :!type "EObjectTypeQuery Enum") true))
  (if _returnvalue
    (`|SpawnActorFromClass` "/Game/Blueprints/Level/Props/BP_BloodPool.BP_BloodPool_C" (`KismetMathLibrary.MakeTransform` (`.Location` (`GameplayStatics.BreakHitResult` _outhit)) (`KismetMathLibrary.MakeRotator` 0.0 0.0 (`KismetMathLibrary.RandomFloatInRange` 0.0 360.0))) "AlwaysSpawn" "MultiplyWithRoot" null (`KismetMathLibrary.RandomFloatInRange` 0.3 0.6) (`KismetMathLibrary.RandomFloatInRange` 8.0 15.0) 20.0 20.0 false null)))