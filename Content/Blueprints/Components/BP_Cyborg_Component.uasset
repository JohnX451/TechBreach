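; BP_Cyborg_Component is an actor component that handles melee attack and death behavior for cyborg enemies.
; A melee call plays an attack montage on the owning EnemyBaseCharacter, then after a short delay damages the player with kinetic melee damage and a hit sound if within range.
; Death casts the owner directly to BP_Enemy_CyborgOperator_01 and calls its Death, a hard reference noted for later replacement with an interface.
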(event `self.MeleeAttackCalled`
  (params (AttackType :type Byte))
  (bind _returnvalue (`GameplayStatics.GetPlayerCharacter` 0))
  (bind _returnvalue_2 (`self.GetOwner`))
  (bind _asenemy_base_character (cast `EnemyBaseCharacter` _returnvalue_2))
  (`Character.PlayAnimMontage` _asenemy_base_character "/Game/Characters/CyborgOperator/Montage_Melee01.Montage_Melee01" 1.0 "None")
  (`KismetSystemLibrary.Delay` 0.4)
  (if (< (`Actor.GetDistanceTo` _returnvalue_2 _returnvalue) 200.0)
    (`GameplayStatics.ApplyDamage` _returnvalue 20.0 (`AIBlueprintHelperLibrary.GetAIController` _returnvalue_2) _returnvalue_2 "/Game/Blueprints/DamageTypes/BP_DT_Weapon_Melee_Kinetic.BP_DT_Weapon_Melee_Kinetic_C")
    (`GameplayStatics.PlaySoundAtLocation` "/Game/Audio/Weapons/Impacts/MS_Weapon_Hit_Melee01.MS_Weapon_Hit_Melee01" (`Actor.K2_GetActorLocation` _returnvalue) (struct) 1.0 1.0 0.0 null null null null)))

(event `self.Death`
  (params (DeathType :type Byte))
  ;[1 1 1] Oh no, ugly. Use Interface later.
  (bind _asbp_enemy_cyborg_operator_01 (cast `/Game/Blueprints/Enemies/BP_Enemy_CyborgOperator_01` (`self.GetOwner`)))
  (`/Game/Blueprints/Enemies/BP_Enemy_CyborgOperator_01.Death` _asbp_enemy_cyborg_operator_01 0))