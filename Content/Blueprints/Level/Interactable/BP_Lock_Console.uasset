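; BP_Lock_Console is an interactable reactor lock console that can be unlocked once through its Use event.
; Construction creates a dynamic screen material on the Cube and sets the initial lock texture.
; When TryUnlocking succeeds, Use notifies the quest component, clears the Cube's tags and custom-depth rendering, swaps the screen texture and plays a confirmation sound.
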(event `self.Use`
  (bind _cube (`self.Cube`))
  (if (not (`self.bIsUnlocked`))
    (bind _returnvalue (`self.TryUnlocking`))
    (if _returnvalue
      (set `self.bIsUnlocked` true)
      (`/Game/Blueprints/QuestSystem/AC_QuestActorComponent.QuestInteraction` (`self.BP_QuestActorComponent`))
      (`KismetArrayLibrary.Array_Clear` (`ActorComponent.ComponentTags` _cube))
      (`PrimitiveComponent.SetRenderCustomDepth` _cube false)
      (`MaterialInstanceDynamic.SetTextureParameterValue` (`self.MatInst`) "Texture" "/Game/Blueprints/Level/Props/Textures/Screens/T_Screen_ReactorLock02.T_Screen_ReactorLock02")
      (`GameplayStatics.PlaySoundAtLocation` "/Game/Audio/Misc/MS_Prop_Console_Yes.MS_Prop_Console_Yes" (`SceneComponent.K2_GetComponentLocation` (`self.Cube`)) (struct) 1.0 1.0 0.0 null null null null))))

(fn `UserConstructionScript`
  (bind _returnvalue (`PrimitiveComponent.CreateDynamicMaterialInstance` (`self.Cube`) 1 "/Game/Materials/Screens/MI_Screen_Default.MI_Screen_Default" "None"))
  (bind _output_get (set `self.MatInst` _returnvalue))
  (`MaterialInstanceDynamic.SetTextureParameterValue` _output_get "Texture" "/Game/Blueprints/Level/Props/Textures/Screens/T_Screen_ReactorLock01.T_Screen_ReactorLock01"))