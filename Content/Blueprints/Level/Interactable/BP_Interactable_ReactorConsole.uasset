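; Interactable reactor console that lets the player restart the reactor core once and restore power to the main elevator.
; On BeginPlay it finds the elevator console, reactor core and turbines by class and sets its popup prompt.
; Use removes the prompt and highlight, advances the quest, fades the core's glow and starts timed reactor and turbine sounds.
; After delays it swaps screen textures, including the info consoles, powers the elevator and calls OnPowerRestored.
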(event `self.SetInteractionPopup`
  (params (bShow :type Boolean))
  (bind _widget (`self.Widget`)
    (:`then`
      (`SceneComponent.SetHiddenInGame` _widget (not bShow) false))
    (:`else`)))

(event `self.ReceiveBeginPlay`
  (`parent.ReceiveBeginPlay`)
  (`KismetSystemLibrary.Delay` 0.2)
  (`|ExecutionSequence`
    (:`then_0`
      (bind _returnvalue (`GameplayStatics.GetActorOfClass` "/Game/Blueprints/Level/Elevators/BP_MainElevator_Console.BP_MainElevator_Console_C"))
      (set `self.ElevatorConsole` _returnvalue))
    (:`then_1`
      (bind _returnvalue_2 (`GameplayStatics.GetActorOfClass` "/Game/Blueprints/Level/Props/BP_ReactorCore.BP_ReactorCore_C"))
      (set `self.ReactorCore` _returnvalue_2))
    (:`then_2`
      (bind _outactors (`GameplayStatics.GetAllActorsOfClass` "/Game/Blueprints/Level/Props/BP_Reactor_Turbine.BP_Reactor_Turbine_C"))
      (set `self.Turbines` _outactors))
    (:`then_3`
      (bind _aswbp_hud_popup_simple (cast `/Game/Blueprints/UI/HUD/WBP_HUD_Popup_Simple` (`WidgetComponent.GetWidget` (`self.Widget`))))
      (`/Game/Blueprints/UI/HUD/WBP_HUD_Popup_Simple.SetText` _aswbp_hud_popup_simple "RESTART REACTOR CORE"))))

(event `self.Use`
  (bind _mesh (`self.Mesh`))
  (`/Engine/EditorBlueprintResources/StandardMacros.DoOnce` false
    (:`Completed`
      (`ActorComponent.K2_DestroyComponent` (`self.Widget`))
      (`self.HandleSound`)
      (`/Game/Blueprints/Level/Props/BP_ReactorCore.FadeOutGlow` (`self.ReactorCore`))
      (`KismetArrayLibrary.Array_Clear` (`ActorComponent.ComponentTags` _mesh))
      (`PrimitiveComponent.SetRenderCustomDepth` _mesh false)
      (`/Game/Blueprints/QuestSystem/AC_QuestActorComponent.QuestInteraction` (`self.BP_QuestActorComponent`))
      (`GameplayStatics.PlaySound2D` "/Game/Audio/Misc/MS_Prop_Console_Yes.MS_Prop_Console_Yes" 1.0 1.0 0.0 null null)
      (bind _returnvalue (`PrimitiveComponent.CreateDynamicMaterialInstance` (`self.Mesh`) 1 "/Game/Materials/Screens/MI_Screen_ReactorConsole_01.MI_Screen_ReactorConsole_01" "None"))
      (bind _output_get (set `self.MatInst` _returnvalue))
      (`MaterialInstanceDynamic.SetTextureParameterValue` _output_get "Texture" "/Game/Blueprints/Level/Props/Textures/Screens/T_Screen_Reactor02.T_Screen_Reactor02")
      (`KismetSystemLibrary.Delay` 10.0)
      (`MaterialInstanceDynamic.SetTextureParameterValue` (`self.MatInst`) "Texture" "/Game/Blueprints/Level/Props/Textures/Screens/T_Screen_Reactor03.T_Screen_Reactor03")
      (bind _elevatorconsole (`self.ElevatorConsole`)
        (:`then`
          (set `/Game/Blueprints/Level/Elevators/BP_MainElevator_Console.bHasPower` true _elevatorconsole)
          (`/Game/Blueprints/Level/Props/BP_Screen_Dynamic.SetScreenTexture` (`self.ReactorInfoConsole`) "/Game/Blueprints/Level/Props/Textures/Screens/T_Screen_ReactorInfo02.T_Screen_ReactorInfo02")
          (`/Game/Blueprints/Level/Props/BP_Screen_Dynamic.SetScreenTexture` (`self.TurbineInfoConsole`) "/Game/Blueprints/Level/Props/Textures/Screens/T_Screen_TurbineInfo02.T_Screen_TurbineInfo02")
          (`KismetSystemLibrary.Delay` 1.0)
          (`self.OnPowerRestored`))
        (:`else`)))))

(event `HandleSound`
  (`|ExecutionSequence`
    (:`then_0`
      (`GameplayStatics.SpawnSoundAtLocation` "/Game/Audio/Environment/MS_Reactor_Start.MS_Reactor_Start" (`self.K2_GetActorLocation`) (struct) 1.0 1.0 0.0 "/Game/Audio/Large_Att.Large_Att" null)
      (`KismetSystemLibrary.Delay` 4.34)
      (`ActorComponent.SetActive` (`self.Audio`) true false))
    (:`then_1`
      (`KismetSystemLibrary.Delay` 5.0)
      (for _array_element (`self.Turbines`)
        (`/Game/Blueprints/Level/Props/BP_Reactor_Turbine.HandleSound` _array_element)))))

(fn `UserConstructionScript`
  (`parent.UserConstructionScript`))