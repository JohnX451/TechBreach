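; Spherical radiation damage volume that reports actors entering and exiting to its damage-volume logic.
; On BeginPlay, the sphere radius drives the max damage distance, post-process blend radius and audio attenuation range, so resizing the sphere scales all three.
; Sphere overlaps register and unregister actors, and toggle a HUD warning when the actor is the player character.
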(event `self.ReceiveBeginPlay`
  (bind _sphereradius (`SphereComponent.SphereRadius` (`self.Sphere`)))
  (bind _returnvalue (* _sphereradius 1.2))
  (`self.SetMaxDamageDistance` _sphereradius)
  (set `PostProcessComponent.BlendRadius` (* _sphereradius 1.25) (`self.PostProcess`))
  (`AudioComponent.AdjustAttenuation` (`self.Audio`) (make `SoundAttenuationSettings` true true false true false true false true false false false false false true "SPATIALIZATION_Default" null 0.0 (struct :`EditorCurveData` (struct :`DefaultValue` 3.4028234663852886e+38 :`PreInfinityExtrap` "RCCE_Constant" :`PostInfinityExtrap` "RCCE_Constant")) (struct :`EditorCurveData` (struct :`DefaultValue` 3.4028234663852886e+38 :`PreInfinityExtrap` "RCCE_Constant" :`PostInfinityExtrap` "RCCE_Constant")) "Linear" "ECC_Visibility" "Linear" "Linear" 0.0 0.0 "OmniDirectional" 200.0 100.0 _returnvalue 20000.0 20000.0 0.0 0.0 30.0 60.0 1.0 1.0 1.0 1.0 1.0 1.0 1.0 1.0 20.0 1.0 0.1 0.3 0.95 400.0 4000.0 0.0 1.0 1.0 100.0 _returnvalue 1.0 (struct :`EditorCurveData` (struct :`DefaultValue` 3.4028234663852886e+38 :`PreInfinityExtrap` "RCCE_Constant" :`PostInfinityExtrap` "RCCE_Constant")) _ (struct :`EditorCurveData` (struct :`DefaultValue` 3.4028234663852886e+38 :`PreInfinityExtrap` "RCCE_Constant" :`PostInfinityExtrap` "RCCE_Constant")) (struct) "Linear" "Sphere" "Continues" -60.0 (100.0 0.0 0.0) 0.0 _returnvalue)))

(event `self.Sphere.OnComponentBeginOverlap`
  (params (OverlappedComponent :type "PrimitiveComponent Object Reference") (OtherActor :type "Actor Object Reference") (OtherComp :type "PrimitiveComponent Object Reference") (OtherBodyIndex :type Integer) (bFromSweep :type Boolean) (SweepResult :type "HitResult Structure (by ref)"))
  (`/Engine/EditorBlueprintResources/StandardMacros.IsValid` OtherActor
    (:`Is Valid`
      (`self.ActorEnteredVolume` OtherActor)
      (if (== OtherActor (`GameplayStatics.GetPlayerCharacter` 0))
        (`/Game/Blueprints/BP_TechFunctions.SetHudWarning` "NewEnumerator0")))))

(event `self.Sphere.OnComponentEndOverlap`
  (params (OverlappedComponent :type "PrimitiveComponent Object Reference") (OtherActor :type "Actor Object Reference") (OtherComp :type "PrimitiveComponent Object Reference") (OtherBodyIndex :type Integer))
  (`/Engine/EditorBlueprintResources/StandardMacros.IsValid` OtherActor
    (:`Is Valid`
      (`self.ActorExitedVolume` OtherActor)
      (if (== OtherActor (`GameplayStatics.GetPlayerCharacter` 0))
        (`/Game/Blueprints/BP_TechFunctions.SetHudWarning` "NewEnumerator0" "Hidden")))))

(fn `UserConstructionScript`)