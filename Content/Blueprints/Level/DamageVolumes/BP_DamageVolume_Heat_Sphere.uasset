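; Sphere-shaped heat damage volume with a post-process effect around it.
; On BeginPlay it sets the post-process blend radius to a quarter of the sphere's radius, so the blend scales with the volume's size.
; Sphere begin and end overlaps forward valid actors to ActorEnteredVolume and ActorExitedVolume, whose logic is defined outside this graph.
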(event `self.ReceiveBeginPlay`
  (set `PostProcessComponent.BlendRadius` (* (`SphereComponent.SphereRadius` (`self.Sphere`)) 0.25) (`self.PostProcess`)))

(event `self.Sphere.OnComponentBeginOverlap`
  (params (OverlappedComponent :type "PrimitiveComponent Object Reference") (OtherActor :type "Actor Object Reference") (OtherComp :type "PrimitiveComponent Object Reference") (OtherBodyIndex :type Integer) (bFromSweep :type Boolean) (SweepResult :type "HitResult Structure (by ref)"))
  (`/Engine/EditorBlueprintResources/StandardMacros.IsValid` OtherActor
    (:`Is Valid`
      (`self.ActorEnteredVolume` OtherActor))))

(event `self.Sphere.OnComponentEndOverlap`
  (params (OverlappedComponent :type "PrimitiveComponent Object Reference") (OtherActor :type "Actor Object Reference") (OtherComp :type "PrimitiveComponent Object Reference") (OtherBodyIndex :type Integer))
  (`/Engine/EditorBlueprintResources/StandardMacros.IsValid` OtherActor
    (:`Is Valid`
      (`self.ActorExitedVolume` OtherActor))))

(fn `UserConstructionScript`)