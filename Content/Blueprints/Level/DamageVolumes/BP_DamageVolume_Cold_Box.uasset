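; BP_DamageVolume_Cold_Box is a box-shaped cold damage volume for levels.
; Box overlaps pass entering and exiting actors to ActorEnteredVolume and ActorExitedVolume, whose logic lives outside this graph.
; The player character's overlaps also show and hide a HUD warning.
; At BeginPlay, the post-process blend radius is scaled from the length of the box extent, so the effect's falloff follows the volume's size.
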(event `self.ReceiveBeginPlay`
  (set `PostProcessComponent.BlendRadius` (* (`KismetMathLibrary.VSize` (`BoxComponent.BoxExtent` (`self.Box`))) 0.25) (`self.PostProcess`)))

(event `self.Box.OnComponentBeginOverlap`
  (params (OverlappedComponent :type "PrimitiveComponent Object Reference") (OtherActor :type "Actor Object Reference") (OtherComp :type "PrimitiveComponent Object Reference") (OtherBodyIndex :type Integer) (bFromSweep :type Boolean) (SweepResult :type "HitResult Structure (by ref)"))
  (`/Engine/EditorBlueprintResources/StandardMacros.IsValid` OtherActor
    (:`Is Valid`
      (`self.ActorEnteredVolume` OtherActor)
      (if (== OtherActor (`GameplayStatics.GetPlayerCharacter` 0))
        (`/Game/Blueprints/BP_TechFunctions.SetHudWarning` "NewEnumerator2")))))

(event `self.Box.OnComponentEndOverlap`
  (params (OverlappedComponent :type "PrimitiveComponent Object Reference") (OtherActor :type "Actor Object Reference") (OtherComp :type "PrimitiveComponent Object Reference") (OtherBodyIndex :type Integer))
  (`/Engine/EditorBlueprintResources/StandardMacros.IsValid` OtherActor
    (:`Is Valid`
      (`self.ActorExitedVolume` OtherActor)
      (if (== OtherActor (`GameplayStatics.GetPlayerCharacter` 0))
        (`/Game/Blueprints/BP_TechFunctions.SetHudWarning` "NewEnumerator2" "Hidden")))))

(fn `UserConstructionScript`)