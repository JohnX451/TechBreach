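; Spherical electricity damage volume that passes actors entering or leaving its sphere to ActorEnteredVolume and ActorExitedVolume, whose logic is not defined here.
; On BeginPlay it scales the post-process blend radius to the sphere, then starts a self-repeating effects loop with randomized delays.
; Each pass spawns sparks and a sound at separately randomized X/Y offsets within the radius, at the sphere's center height.
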(event `self.ReceiveBeginPlay`
  (set `PostProcessComponent.BlendRadius` (* (`SphereComponent.SphereRadius` (`self.Sphere`)) 0.25) (`self.PostProcess`))
  (`self.PlayEffects`))

(event `PlayEffects`
  (`self.SpawnEffects`)
  (`KismetSystemLibrary.Delay` (`self.EffectDelay`))
  (set `self.EffectDelay` (`KismetMathLibrary.RandomFloatInRange` 0.05 1.0))
  (`self.PlayEffects`))

(event `self.Sphere.OnComponentBeginOverlap`
  (params (OverlappedComponent :type "PrimitiveComponent Object Reference") (OtherActor :type "Actor Object Reference") (OtherComp :type "PrimitiveComponent Object Reference") (OtherBodyIndex :type Integer) (bFromSweep :type Boolean) (SweepResult :type "HitResult Structure (by ref)"))
  (`/Engine/EditorBlueprintResources/StandardMacros.IsValid` OtherActor
    (:`Is Valid`
      (`self.ActorEnteredVolume` OtherActor))))

(event `self.Sphere.OnComponentEndOverlap`
  (params (OverlappedComponent :type "PrimitiveComponent Object Reference") (OtherActor :type "Actor Object Reference") (OtherComp :type "PrimitiveComponent Object Reference") (OtherBodyIndex :type Integer))
  (`/Engine/EditorBlueprintResources/StandardMacros.IsValid` OtherActor
    (:`Is Valid`
      (`self.ActorExitedVolume` OtherActor))))

(fn `SpawnEffects`
  (bind _sphere (`self.Sphere`))
  (bind (_returnvalue_x _returnvalue_y _returnvalue_z) (`KismetMathLibrary.BreakVector` (`SceneComponent.K2_GetComponentLocation` _sphere)))
  (bind _sphereradius (`SphereComponent.SphereRadius` _sphere))
  (bind _returnvalue (* _sphereradius -1.0))
  (bind _returnvalue_2 (`KismetMathLibrary.MakeVector` (+ _returnvalue_x (`KismetMathLibrary.RandomFloatInRange` _returnvalue _sphereradius)) (+ _returnvalue_y (`KismetMathLibrary.RandomFloatInRange` _returnvalue _sphereradius)) _returnvalue_z))
  (`GameplayStatics.SpawnEmitterAtLocation` "/Game/ThirdParty/Realistic_Starter_VFX_Pack_Vol2/Particles/TechBreach/P_Sparks_Env_01.P_Sparks_Env_01" _returnvalue_2 (`KismetMathLibrary.MakeRotator` 0.0 0.0 (`KismetMathLibrary.RandomFloatInRange` 0.0 359.0)))
  (`GameplayStatics.PlaySoundAtLocation` "/Game/Audio/Environment/MS_Env_Sparks_01.MS_Env_Sparks_01" _returnvalue_2 (struct) 1.0 1.0 0.0 "/Game/Audio/EnemyFootsteps_Att.EnemyFootsteps_Att" null null null)
  (return))

(fn `UserConstructionScript`)