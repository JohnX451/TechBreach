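; BP_Lock_Code is an access lock for doors that displays its required key level, set by the construction script from UnlockKey.
; Using it while locked and non-hackable calls TryUnlocking, and a failure triggers a quest interaction through a DoOnce.
; UnlockConsole clears the Lock's tags, custom depth and text, then turns its light green through a dynamic material instance.
; A helper event plays sounds at the Lock's location.
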(event `self.Use`
  (if (`self.bIsLocked`)
    (if (not (`self.bIsHackable`))
      (bind _returnvalue (`self.TryUnlocking`))
      (if (not _returnvalue)
        (`/Engine/EditorBlueprintResources/StandardMacros.DoOnce` false
          (:`Completed`
            (`/Game/Blueprints/QuestSystem/BP_QuestActorComponent.QuestInteraction` (`self.BP_QuestActorComponent`))))))))

(event `self.UnlockConsole`
  (bind _lock (`self.Lock`))
  (`KismetArrayLibrary.Array_Clear` (`ActorComponent.ComponentTags` _lock))
  (`PrimitiveComponent.SetRenderCustomDepth` _lock false)
  (`TextRenderComponent.K2_SetText` (`self.LockText`) "")
  (bind _returnvalue (`PrimitiveComponent.CreateDynamicMaterialInstance` (`self.Lock`) 1 "/Game/Materials/Doors/MI_Light_LockCode.MI_Light_LockCode" "None"))
  (`MaterialInstanceDynamic.SetVectorParameterValue` _returnvalue "ColorLight" (struct :`G` 1.0 :`B` 0.13744 :`A` 1.0)))

(event `self.PlaySound`
  (params (Sound :type "SoundBase Object Reference"))
  (`GameplayStatics.PlaySoundAtLocation` Sound (`SceneComponent.K2_GetComponentLocation` (`self.Lock`)) (struct) 1.0 1.0 0.0 null null null null))

(fn `UserConstructionScript`
  (`TextRenderComponent.K2_SetText` (`self.LockText`) (`|FormatText` "ACCESS LOCK \n--LEVEL:{a}" (`self.UnlockKey`))))