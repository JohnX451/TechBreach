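; Interactable crawlspace hatch that shows an "OPEN HATCH" popup widget and opens when used.
; Popup visibility and Use are gated by IsOpen, which this graph never sets.
; Use clears the Door's tags and custom depth, hides the popup, plays a vent sound and runs the OpenHatch timeline to move the Door along relative Z.
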(event `self.ReceiveBeginPlay`
  (bind _aswbp_hud_popup_simple (cast `/Game/Blueprints/UI/HUD/WBP_HUD_Popup_Simple` (`WidgetComponent.GetWidget` (`self.Widget`))))
  (`/Game/Blueprints/UI/HUD/WBP_HUD_Popup_Simple.SetText` _aswbp_hud_popup_simple "OPEN HATCH"))

(event `self.SetInteractionPopup`
  (params (bShow :type Boolean))
  (if (not (`self.bIsOpen`))
    (`SceneComponent.SetHiddenInGame` (`self.Widget`) (not bShow) false)))

(event `self.Use`
  (bind _door (`self.Door`))
  (if (not (`self.bIsOpen`))
    (`KismetArrayLibrary.Array_Clear` (`ActorComponent.ComponentTags` _door))
    (`PrimitiveComponent.SetRenderCustomDepth` _door false)
    (`GameplayStatics.SpawnSoundAtLocation` "/Game/Audio/Misc/MS_Prop_Vent_Open.MS_Prop_Vent_Open" (`SceneComponent.K2_GetComponentLocation` (`self.DefaultSceneRoot`)) (struct) 1.0 1.0 0.0 null null)
    (`SceneComponent.SetHiddenInGame` (`self.Widget`) true false)
    (bind (_direction _locationz) (`Timeline|OpenHatch` :!via `PlayFromStart`)
      (:`Update`
        (`SceneComponent.K2_SetRelativeLocation` (`self.Door`) (`KismetMathLibrary.MakeVector` 0.0 0.0 _locationz) false false)))))

(fn `UserConstructionScript`)