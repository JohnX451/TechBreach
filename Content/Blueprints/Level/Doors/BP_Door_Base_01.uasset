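; Base interactable sliding door that can be locked, unlocked or hacked, with button lights colored by lock state.
; Use calls OpenDoorAction when unlocked; otherwise it tries unlocking, then a timed hack scaled by the player's HackSpeed stat with HUD progress.
; Successful unlocks play a sound and report the door's ObjectiveID to the player for quests.
; OpenDoor and CloseDoor drive a timeline on the door's Y offset, toggle its highlight tag, and opening calls PrimeForClosing.
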(event `self.Use`
  (bind _returnvalue (`self.GetComponentByClass` (`GameplayStatics.GetPlayerCharacter` 0) "/Game/Blueprints/Components/BP_StatsComponent.BP_StatsComponent_C"))
  (bind _returnvalue_2 (* (`self.BaseHackDuration`) (`BlueprintMapLibrary.Map_Find` (`StatsComponent.CurrentAttributeValues` _returnvalue) "HackSpeed")))
  (if (`self.bIsLocked`)
    (bind _returnvalue_3 (`self.TryUnlocking`))
    (if _returnvalue_3
      (`self.Set Button Colors`)
      (`GameplayStatics.PlaySoundAtLocation` "/Game/Audio/Doors/MS_Prop_Door_Unlock_01.MS_Prop_Door_Unlock_01" (`SceneComponent.K2_GetComponentLocation` (`self.Frame`)) (struct) 1.0 1.0 0.0 null null null null)
      ;[1 1 1] Quest Notification
      (bind _asbp_player_character (cast `/Game/Blueprints/Player/BP_PlayerCharacter` (`GameplayStatics.GetPlayerCharacter` 0)))
      (`/Game/Blueprints/Player/BP_PlayerCharacter.OnObjectiveIDCalled` _asbp_player_character (`self.ObjectiveID`) 1)
      (else
        (`KismetSystemLibrary.PrintString` "Door is locked!")
        ;[1 1 1] Hackable Objects might need to become a BaseClass on its own?
        (if (and (`self.bIsHackable`) (not (`self.bIsHackInProgress`)))
          (bind _returnvalue_4 (`self.TryHackingUnlock`))
          (if _returnvalue_4
            (`KismetSystemLibrary.PrintString` "Starting hack")
            (set `self.bIsHackInProgress` true)
            (`/Game/Blueprints/Demo/UIDemo/WBP_Demo_HackingProgress.StartHacking` (`/Game/Blueprints/Demo/UIDemo/WBP_Demo_HUD.HackingProgress` (`/Game/Blueprints/Components/BP_StatsComponent.PlayerHUD` _returnvalue)) _returnvalue_2)
            (`KismetSystemLibrary.Delay` _returnvalue_2)
            (set `self.bIsLocked` false)
            (`self.Set Button Colors`)
            (`GameplayStatics.PlaySoundAtLocation` "/Game/Audio/Doors/MS_Prop_Door_Unlock_01.MS_Prop_Door_Unlock_01" (`SceneComponent.K2_GetComponentLocation` (`self.Frame`)) (struct) 1.0 1.0 0.0 null null null null)
            ;[1 1 1] Quest Notification
            (bind _asbp_player_character_2 (cast `/Game/Blueprints/Player/BP_PlayerCharacter` (`GameplayStatics.GetPlayerCharacter` 0)))
            (`/Game/Blueprints/Player/BP_PlayerCharacter.OnObjectiveIDCalled` _asbp_player_character_2 (`self.ObjectiveID`) 1)
            (else
              (`GameplayStatics.PlaySoundAtLocation` "/Game/Audio/Doors/MS_Prop_Door_Locked_01.MS_Prop_Door_Locked_01" (`SceneComponent.K2_GetComponentLocation` (`self.Frame`)) (struct) 1.0 1.0 0.0 null null null null :!label _label)
              (`KismetSystemLibrary.PrintString` "Door Hack failed!")))
          (else
            (goto _label)))))
    (else
      (`self.OpenDoorAction`))))

(event `self.SetInteractionPopup`
  (params (bShow :type Boolean)))

(event `self.OpenDoor`
  (bind _door (`self.Door`))
  (`GameplayStatics.PlaySoundAtLocation` "/Game/Audio/Doors/MS_Prop_Door_Open_01.MS_Prop_Door_Open_01" (`SceneComponent.K2_GetComponentLocation` (`self.Frame`)) (struct) 1.0 1.0 0.0 null null null null)
  (`self.PrimeForClosing`)
  (`TimelineComponent.SetPlayRate` (`self.TimelineOpenDoor`) (`self.OpenSpeedSeconds`))
  (`KismetArrayLibrary.Array_Clear` (`ActorComponent.ComponentTags` _door))
  (`PrimitiveComponent.SetRenderCustomDepth` _door false)
  (bind (_direction _yoffset) (`Timeline|TimelineOpenDoor` :`NewTime` 1.0 :!label _label_2)
    (:`Update`
      (`SceneComponent.K2_SetRelativeLocation` (`self.Door`) (`KismetMathLibrary.MakeVector` 0.0 _yoffset) false false))))

(event `self.CloseDoor`
  (`GameplayStatics.PlaySoundAtLocation` "/Game/Audio/Doors/MS_Prop_Door_Close_01.MS_Prop_Door_Close_01" (`SceneComponent.K2_GetComponentLocation` (`self.Frame`)) (struct) 1.0 1.0 0.0 null null null null)
  (`TimelineComponent.SetPlayRate` (`self.TimelineOpenDoor`) (`self.CloseSpeedSeconds`))
  (set `ActorComponent.ComponentTags` (`|MakeArray` "highlightable" :!type "Name") (`self.Door`))
  (goto _label_2 :!via `Reverse`))

(fn `Set Button Colors`
  (bind _returnvalue (`KismetMathLibrary.SelectColor` (`self.ColorLocked`) (`self.ColorUnlocked`) (`self.bIsLocked`)))
  (`MaterialInstanceDynamic.SetVectorParameterValue` (`self.Button1Mat`) "Color" _returnvalue)
  (`MaterialInstanceDynamic.SetVectorParameterValue` (`self.Button2Mat`) "Color" _returnvalue))

(fn `UserConstructionScript`
  (bind _returnvalue (`PrimitiveComponent.CreateDynamicMaterialInstance` (`self.Button1`) 1 "/Game/Materials/MI_Light_Blue.MI_Light_Blue" "None"))
  (set `self.Button1Mat` _returnvalue)
  (bind _returnvalue_2 (`PrimitiveComponent.CreateDynamicMaterialInstance` (`self.Button2`) 1 "/Game/Materials/MI_Light_Blue.MI_Light_Blue" "None"))
  (set `self.Button2Mat` _returnvalue_2)
  (`self.Set Button Colors`))