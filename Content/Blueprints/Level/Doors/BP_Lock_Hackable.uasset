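; BP_Lock_Hackable is a door lock that the player opens by hacking, with its required hacking level displayed as override text.
; On use, a successful TryHackingUnlock starts the player HUD's hacking progress, with base duration multiplied by the player's HackSpeed attribute.
; After that duration plus a short fixed padding, it calls UnlockConsoleAction.
; The UnlockConsole event clears the lock's tags, outline depth and text, and turns its light green via a dynamic material.
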(event `self.Use`
  (bind _returnvalue (`self.GetComponentByClass` (`GameplayStatics.GetPlayerCharacter` 0) "/Game/Blueprints/Components/BP_StatsComponent.BP_StatsComponent_C"))
  (bind _returnvalue_2 (* (`self.BaseHackDuration`) (`BlueprintMapLibrary.Map_Find` (`StatsComponent.CurrentAttributeValues` _returnvalue) "HackSpeed")))
  (if (`self.bIsLocked`)
    (if (and (`self.bIsHackable`) (not (`self.bIsHackInProgress`)))
      (bind _returnvalue_3 (`self.TryHackingUnlock`))
      (if _returnvalue_3
        (set `self.bIsHackInProgress` true)
        (`/Game/Blueprints/UI/WBP_HUD_Hacking.StartHacking` (`/Game/Blueprints/Demo/UIDemo/WBP_Demo_HUD.HackingProgress` (`/Game/Blueprints/Components/BP_StatsComponent.PlayerHUD` _returnvalue)) _returnvalue_2 (`self.SystemName`) (`self.RequiredHackingLevel`))
        (`KismetSystemLibrary.Delay` (+ _returnvalue_2 0.9 0.9))
        (`self.UnlockConsoleAction`)))))

(event `self.UnlockConsole`
  (bind _lock (`self.Lock`))
  (`KismetArrayLibrary.Array_Clear` (`ActorComponent.ComponentTags` _lock))
  (`PrimitiveComponent.SetRenderCustomDepth` _lock false)
  (`TextRenderComponent.K2_SetText` (`self.LockText`) "")
  (bind _returnvalue (`PrimitiveComponent.CreateDynamicMaterialInstance` (`self.Lock`) 1 "/Game/Materials/Doors/MI_Light_LockCode.MI_Light_LockCode" "None"))
  (`MaterialInstanceDynamic.SetVectorParameterValue` _returnvalue "ColorLight" (struct :`G` 1.0 :`B` 0.13744 :`A` 1.0)))

(event `self.PlaySound`
  (params (Sound :type "SoundBase Object Reference"))
  (`GameplayStatics.PlaySoundAtLocation` Sound (`SceneComponent.K2_GetComponentLocation` (`self.Lock`)) (struct) 1.0 1.0 0.0 null null null null))

(fn `UserConstructionScript`
  (`TextRenderComponent.K2_SetText` (`self.LockText`) (`|FormatText` "SEC-OVERRIDE \n--MANUAL \n--REQ-V:{a}" (`KismetStringLibrary.Conv_ByteToString` (`self.RequiredHackingLevel`)))))