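; BP_Door_Double_A is a double sliding door that opens on use, or automatically when a cyborg operator enemy overlaps it, unless locked.
; Use ignores input while busy and plays a locked sound when locked, otherwise calling OpenDoorAction.
; A timeline slides both panels apart along Y and reverses to close, with sounds at the frame.
; Opening clears highlight tags and custom depth, and closing restores the tags.
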(event `self.PlaySound`
  (params (Sound :type "SoundBase Object Reference"))
  (`GameplayStatics.PlaySoundAtLocation` Sound (`SceneComponent.K2_GetComponentLocation` (`self.Frame`)) (struct) 1.0 1.0 0.0 null null null null))

(event `self.Use`
  (if (`self.bIsBusy`)
    _
    (elif (`self.bIsLocked`)
      (`GameplayStatics.PlaySoundAtLocation` (`self.SoundLocked`) (`SceneComponent.K2_GetComponentLocation` (`self.Frame`)) (struct) 1.0 1.0 0.0 null null null null)
      (else
        (`self.OpenDoorAction`)))))

(event `self.OpenDoor`
  (bind _door1 (`self.Door1`))
  (set `self.bIsBusy` true)
  (`GameplayStatics.PlaySoundAtLocation` (`self.SoundOpen`) (`SceneComponent.K2_GetComponentLocation` (`self.Frame`)) (struct) 1.0 1.0 0.0 null null null null)
  (`self.PrimeForClosing`)
  (`TimelineComponent.SetPlayRate` (`self.TimelineOpenDoor`) (`self.OpenSpeedSeconds`))
  (`KismetArrayLibrary.Array_Clear` (`ActorComponent.ComponentTags` _door1))
  (`KismetArrayLibrary.Array_Clear` (`ActorComponent.ComponentTags` (`self.Door2`)))
  (`PrimitiveComponent.SetRenderCustomDepth` _door1 false)
  (`PrimitiveComponent.SetRenderCustomDepth` (`self.Door2`) false)
  (bind (_direction _yoffset) (`Timeline|TimelineOpenDoor` :`NewTime` 1.0 :!label _label)
    (:`Update`
      (`SceneComponent.K2_SetRelativeLocation` (`self.Door1`) (`KismetMathLibrary.MakeVector` 0.0 (* _yoffset 130.0)) false false)
      (`SceneComponent.K2_SetRelativeLocation` (`self.Door2`) (`KismetMathLibrary.MakeVector` 0.0 (* _yoffset -110.0)) false false))))

(event `self.CloseDoor`
  (bind _array (`|MakeArray` "highlightable" :!type "Name"))
  (`GameplayStatics.PlaySoundAtLocation` (`self.SoundClose`) (`SceneComponent.K2_GetComponentLocation` (`self.Frame`)) (struct) 1.0 1.0 0.0 null null null null)
  (`TimelineComponent.SetPlayRate` (`self.TimelineOpenDoor`) (`self.CloseSpeedSeconds`))
  (set `ActorComponent.ComponentTags` _array (`self.Door1`))
  (set `ActorComponent.ComponentTags` _array (`self.Door2`))
  (set `self.bIsBusy` false)
  (goto _label :!via `Reverse`))

(event `self.ReceiveActorBeginOverlap`
  (params (OtherActor :type "Actor Object Reference"))
  (if (and (== (`GameplayStatics.GetObjectClass` OtherActor) "/Game/Blueprints/Enemies/BP_Enemy_CyborgOperator_01.BP_Enemy_CyborgOperator_01_C") (not (`self.bIsLocked`)))
    (`self.OpenDoorAction`)))

(fn `UserConstructionScript`)