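; Security door that slides along Z, opened by using it or automatically when an actor with a Cyborg component overlaps it while unlocked.
; Using it while locked plays a locked sound; otherwise both triggers call OpenDoorAction.
; OpenDoor and CloseDoor run one timeline forward or in reverse with separate play rates and sounds.
; Opening removes the door's highlight tag and custom depth, and closing restores the tag.
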(event `self.PlaySound`
  (params (Sound :type "SoundBase Object Reference"))
  (`GameplayStatics.PlaySoundAtLocation` Sound (`SceneComponent.K2_GetComponentLocation` (`self.Frame`)) (struct) 1.0 1.0 0.0 null null null null))

(event `self.Use`
  (if (`self.bIsBusy`)
    _
    (elif (`self.bIsLocked`)
      (`GameplayStatics.PlaySoundAtLocation` (`self.SoundLocked`) (`SceneComponent.K2_GetComponentLocation` (`self.Frame`)) (struct) 1.0 1.0 0.0 null null null null)
      (else
        (`self.OpenDoorAction`)))))

(event `self.OpenDoor`
  (bind _door (`self.Door`))
  (set `self.bIsBusy` true)
  (`GameplayStatics.PlaySoundAtLocation` (`self.SoundOpen`) (`SceneComponent.K2_GetComponentLocation` (`self.Frame`)) (struct) 1.0 1.0 0.0 null null null null)
  (`self.PrimeForClosing`)
  (`TimelineComponent.SetPlayRate` (`self.TimelineOpenDoor`) (`self.OpenSpeedSeconds`))
  (`KismetArrayLibrary.Array_Clear` (`ActorComponent.ComponentTags` _door))
  (`PrimitiveComponent.SetRenderCustomDepth` _door false)
  (bind (_direction _zoffset) (`Timeline|TimelineOpenDoor` :`NewTime` 1.0 :!label _label)
    (:`Update`
      (`SceneComponent.K2_SetRelativeLocation` (`self.Door`) (`KismetMathLibrary.MakeVector` 0.0 0.0 _zoffset) false false))))

(event `self.CloseDoor`
  (`GameplayStatics.PlaySoundAtLocation` (`self.SoundClose`) (`SceneComponent.K2_GetComponentLocation` (`self.Frame`)) (struct) 1.0 1.0 0.0 null null null null)
  (`TimelineComponent.SetPlayRate` (`self.TimelineOpenDoor`) (`self.CloseSpeedSeconds`))
  (set `ActorComponent.ComponentTags` (`|MakeArray` "highlightable" :!type "Name") (`self.Door`))
  (set `self.bIsBusy` false)
  (goto _label :!via `Reverse`))

(event `self.ReceiveActorBeginOverlap`
  (params (OtherActor :type "Actor Object Reference"))
  (if (and (`KismetSystemLibrary.IsValid` (`self.GetComponentByClass` OtherActor "/Game/Blueprints/Components/AC_Cyborg_Component.AC_Cyborg_Component_C")) (not (`self.bIsLocked`)))
    (`self.OpenDoorAction`)))

(fn `UserConstructionScript`)