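; BP_Screen_Dynamic is a level prop screen whose displayed texture can be changed at runtime.
; The construction script creates a dynamic instance of MI_Screen_Default on the static mesh's second material slot and applies the default texture, plus an optional pixel intensity override.
; SetScreenTexture swaps the texture parameter on that stored material instance.
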(fn `SetScreenTexture`
  (params (Texture :type "Texture Object Reference"))
  (`MaterialInstanceDynamic.SetTextureParameterValue` (`self.MatInst`) "Texture" Texture))

(fn `UserConstructionScript`
  (bind _returnvalue (`PrimitiveComponent.CreateDynamicMaterialInstance` (`self.StaticMesh`) 1 "/Game/Materials/Screens/MI_Screen_Default.MI_Screen_Default" "None"))
  (bind _output_get (set `self.MatInst` _returnvalue))
  (`MaterialInstanceDynamic.SetTextureParameterValue` _output_get "Texture" (`self.DefaultTexture`))
  (if (`self.bSetPixelIntensity`)
    (`MaterialInstanceDynamic.SetScalarParameterValue` (`self.MatInst`) "PixelIntensity" (`self.PixelIntensity`))))