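; Blood pool prop that uses a decal to show blood spreading out after it spawns.
; On BeginPlay a timeline, with play rate set from TimeToMaxScale, drives the decal's uniform world scale by a curve multiplied by MaxScale.
; The construction script optionally sets a delayed decal fade-out that destroys the actor when it finishes.
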(event `self.ReceiveBeginPlay`
  (`TimelineComponent.SetPlayRate` (`self.Timeline_GrowPool`) (/ 1.0 (`self.TimeToMaxScale`)))
  (bind (_direction _worldscalecoef) (`Timeline|Timeline_GrowPool` :!via `PlayFromStart`)
    (:`Update`
      (bind _returnvalue (* _worldscalecoef (`self.MaxScale`)))
      (`SceneComponent.SetWorldScale3D` (`self.Decal`) (`KismetMathLibrary.MakeVector` _returnvalue _returnvalue _returnvalue)))))

(fn `UserConstructionScript`
  (if (`self.bFadeOut`)
    (`DecalComponent.SetFadeOut` (`self.Decal`) (`self.FadeStartDelay`) (`self.FadeDuration`) true)))