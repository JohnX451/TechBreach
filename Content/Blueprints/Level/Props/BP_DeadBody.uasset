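; Dead body prop whose skeletal mesh, material and hidden bones are set per instance.
; The construction script applies the mesh asset and material, then hides each bone in a list.
; On BeginPlay it waits a few seconds, then disables the skeletal mesh component's tick.
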(event `self.ReceiveBeginPlay`
  (`KismetSystemLibrary.Delay` 4.0)
  (`ActorComponent.SetComponentTickEnabled` (`self.SkeletalMesh`) false))

(fn `UserConstructionScript`
  (bind _skeletalmesh (`self.SkeletalMesh`))
  (`SkeletalMeshComponent.SetSkeletalMeshAsset` _skeletalmesh (`self.MeshAsset`))
  (`PrimitiveComponent.SetMaterial` _skeletalmesh 0 (`self.MaterialAsset`))
  (for _array_element (`self.BonesToHide`)
    (`SkinnedMeshComponent.HideBoneByName` (`self.SkeletalMesh`) _array_element "PBO_None")))