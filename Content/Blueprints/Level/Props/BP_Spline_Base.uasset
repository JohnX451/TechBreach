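; Base spline prop Blueprint that lays a configurable mesh along a spline.
; The construction script splits the spline into whole SectionLength segments and adds an X-forward spline mesh component per segment, with configurable collision; any leftover length stays uncovered.
; Helper functions supply each segment's local start and end positions and tangents by distance, clamping tangent size to SectionLength.
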(fn `GetEndPositionAndTangent`
  (params (Index :type Integer))
  (returns (Position :type "Vector Structure") (Tangent :type "Vector Structure"))
  (bind _spline (`self.Spline`))
  (bind _returnvalue (* (+ Index 1) (`self.SectionLength`)))
  (return (`SplineComponent.GetLocationAtDistanceAlongSpline` _spline _returnvalue "Local") (`KismetMathLibrary.ClampVectorSize` (`SplineComponent.GetTangentAtDistanceAlongSpline` _spline _returnvalue "Local") 0.0 (`self.SectionLength`))))

(fn `GetStartPositionAndTangent`
  (params (Index :type Integer))
  (returns (Position :type "Vector Structure") (Tangent :type "Vector Structure"))
  (bind _spline (`self.Spline`))
  (bind _returnvalue (* Index (`self.SectionLength`)))
  (return (`SplineComponent.GetLocationAtDistanceAlongSpline` _spline _returnvalue "Local") (`KismetMathLibrary.ClampVectorSize` (`SplineComponent.GetTangentAtDistanceAlongSpline` _spline _returnvalue "Local") 0.0 (`self.SectionLength`))))

(fn `UserConstructionScript`
  (locals (LoopIndex :type Integer))
  (bind _loopindex (`local.LoopIndex`))
  (for _index (range (`KismetMathLibrary.FTrunc` (/ (`SplineComponent.GetSplineLength` (`self.Spline`)) (`self.SectionLength`))))
    (set `local.LoopIndex` _index)
    (bind _returnvalue (`AddComponent|NODE_AddSplineMeshComponent-0`))
    (`StaticMeshComponent.SetStaticMesh` _returnvalue (`self.SplineMesh`))
    (`SplineMeshComponent.SetForwardAxis` _returnvalue "X" true)
    (bind (_position _tangent) (`self.GetStartPositionAndTangent` _loopindex))
    (bind (_position_2 _tangent_2) (`self.GetEndPositionAndTangent` _loopindex))
    (`SplineMeshComponent.SetStartAndEnd` _returnvalue _position _tangent _position_2 _tangent_2 true)
    (`PrimitiveComponent.SetCollisionEnabled` _returnvalue (`self.CollisionEnabled`))))