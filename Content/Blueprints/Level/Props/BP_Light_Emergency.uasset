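; Emergency light prop with an emissive mesh and an optional point light that can blink.
; The construction script creates a dynamic material instance from the shared color and intensity, then configures the point light or destroys it when no light source is wanted.
; When blinking is enabled, BeginPlay starts a self-calling delay loop that uses SetLightEnabled to toggle emissive strength and light visibility together.
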(event `self.ReceiveBeginPlay`
  (if (`self.bIsBlinking`)
    (`self.BlinkLoop`)))

(event `BlinkLoop`
  (if (`self.bIsBlinking`)
    (`KismetSystemLibrary.Delay` 1.0)
    (`self.SetLightEnabled` false)
    (`KismetSystemLibrary.Delay` 0.5)
    (`self.SetLightEnabled` true)
    (`self.BlinkLoop`)))

(fn `SetLightEnabled`
  (params (bNewState :type Boolean))
  (if bNewState
    (`MaterialInstanceDynamic.SetScalarParameterValue` (`self.MaterialInstance`) "EmissiveStrength" (`self.LightIntensity`))
    (if (`self.bUseLightSource`)
      (`SceneComponent.SetHiddenInGame` (`self.PointLight`) false false))
    (else
      (`MaterialInstanceDynamic.SetScalarParameterValue` (`self.MaterialInstance`) "EmissiveStrength" 0.0)
      (if (`self.bUseLightSource`)
        (`SceneComponent.SetHiddenInGame` (`self.PointLight`) true false)))))

(fn `UserConstructionScript`
  (bind _pointlight (`self.PointLight`))
  (bind _returnvalue (`PrimitiveComponent.CreateDynamicMaterialInstance` (`self.LightMesh`) 0 "/Game/Materials/Props/MI_Light_Emergency.MI_Light_Emergency" "None"))
  (bind _output_get (set `self.MaterialInstance` _returnvalue))
  (`MaterialInstanceDynamic.SetScalarParameterValue` _output_get "EmissiveStrength" (`self.LightIntensity`))
  (`MaterialInstanceDynamic.SetVectorParameterValue` (`self.MaterialInstance`) "EmissiveTint" (`self.LightColor`))
  (if (`self.bUseLightSource`)
    (`LightComponentBase.SetCastShadows` _pointlight (`self.bCastShadow`))
    (`LightComponent.SetLightColor` _pointlight (`self.LightColor`) true)
    (`LightComponent.SetIntensity` _pointlight (* (`self.LightIntensity`) 500.0))
    (else
      (`ActorComponent.K2_DestroyComponent` (`self.PointLight`)))))