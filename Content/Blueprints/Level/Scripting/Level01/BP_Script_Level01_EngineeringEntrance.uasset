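; Level 01 scripted trigger for the engineering entrance that plays a one-time bleed-out death on a victim mesh when the player overlaps it.
; It plays a slow bleed-out animation, then after a timed delay switches the mesh to physics simulation for a ragdoll collapse.
; A blood pool actor spawns under the victim's head bone at a fixed floor height.
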(event `self.ReceiveBeginPlay`)

(event `self.ReceiveActorBeginOverlap`
  (params (OtherActor :type "Actor Object Reference"))
  (if (== OtherActor (`GameplayStatics.GetPlayerCharacter` 0))
    (`/Engine/EditorBlueprintResources/StandardMacros.DoOnce` false
      (:`Completed`
        (`self.StartBleedingOut`)))))

(event `StartBleedingOut`
  (bind _skeletalmeshcomponent (`SkeletalMeshActor.SkeletalMeshComponent` (`self.VictimMesh`)))
  (bind _returnvalue (`SkinnedMeshComponent.GetBoneTransform` (`SkeletalMeshActor.SkeletalMeshComponent` (`self.VictimMesh`)) "head" "RTS_World"))
  (`SkeletalMeshComponent.PlayAnimation` _skeletalmeshcomponent "/Game/ThirdParty/DeathAnims/Deaths_Shot_Slow_Bleedout.Deaths_Shot_Slow_Bleedout" false)
  (`KismetSystemLibrary.Delay` 6.1)
  (`PrimitiveComponent.SetSimulatePhysics` _skeletalmeshcomponent true)
  (`|SpawnActorFromClass` "/Game/Blueprints/Level/Props/BP_BloodPool.BP_BloodPool_C" (`KismetMathLibrary.MakeTransform` (`KismetMathLibrary.MakeVector` (.x (.location _returnvalue)) (.y (.location _returnvalue)) -2250.0)) "Undefined" "MultiplyWithRoot" null 0.55 10.0 20.0 20.0 false null))

(fn `UserConstructionScript`)