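; Level 01 script actor that drives the story: voiced HUD messages from Samuel Grayson and Aurora, plus quest progression.
; On BeginPlay, after a short delay, it binds to doors, triggers, the servo armature, reactor console and main elevator.
; Most story beats fire once, and Aurora's message waits for restored power.
; It also unlocks the surgery door, spawns the elevator ambush and shows the success screen when the elevator starts.
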(event `self.ReceiveBeginPlay`
  (`KismetSystemLibrary.Delay` 0.2)
  (add `/Game/Blueprints/Level/Doors/BP_Door_Double_A.OnUnsuccessfulOpen` (`self.CorridorDoor`) (`|CreateDelegate` :!event `QuestAccessLock`))
  (add `/Game/Blueprints/Level/Doors/BP_Lock_Code.OnUnsuccessfulUnlock` (`self.CooridorAccessLock`) (`|CreateDelegate` :!event `QuestAccessLock`))
  (add `/Game/Blueprints/Level/Doors/BP_Door_Standard_A.OnUnsuccessfulOpen` (`self.SurgeryDoor`) (`|CreateDelegate` :!event `QuestSurgeryDoor`))
  (add `/Game/Blueprints/Level/Scripting/BP_PlayerTrigger.OnTriggerActivated` (`self.TriggerVentCorridor`) (`|CreateDelegate` :!event `VentTrigger`))
  (add `/Game/Blueprints/Level/Scripting/BP_PlayerTrigger.OnTriggerActivated` (`self.TriggerVent`) (`|CreateDelegate` :!event `VentTrigger`))
  (bind _returnvalue (`GameplayStatics.GetActorOfClass` "/Game/Blueprints/Level/Interactable/BP_Interactable_ReactorConsole.BP_Interactable_ReactorConsole_C"))
  (add `/Game/Blueprints/Level/Interactable/BP_Interactable_ReactorConsole.OnPowerRestored` _returnvalue (`|CreateDelegate` :!event `PowerRestored`))
  (bind _returnvalue_2 (`GameplayStatics.GetActorOfClass` "/Game/Blueprints/Level/Elevators/BP_MainElevator_Console.BP_MainElevator_Console_C"))
  (add `/Game/Blueprints/Level/Elevators/BP_MainElevator_Console.OnActivatedNoPower` _returnvalue_2 (`|CreateDelegate` :!event `ElevatorTriggered`))
  (add `/Game/Blueprints/Level/Elevators/BP_MainElevator_Console.OnElevatorStarting` _returnvalue_2 (`|CreateDelegate` :!event `ElevatorStarting`))
  (bind _returnvalue_3 (`GameplayStatics.GetActorOfClass` "/Game/Blueprints/Level/Elevators/BP_MainElevator_01.BP_MainElevator_01_C"))
  (bind _output_get (set `self.MainElevator` _returnvalue_3))
  (add `/Game/Blueprints/Level/Elevators/BP_MainElevator_01.OnDoorsOpenedAfterPower` _output_get (`|CreateDelegate` :!event `PoweredElevatorOpened`))
  (add `/Game/Blueprints/Level/Scripting/BP_PlayerTrigger.OnTriggerActivated` (`self.TriggerAurora`) (`|CreateDelegate` :!event `ReceiveMessageFromAurora`))
  (add `/Game/Blueprints/Items/Modules/BP_ImplantItem_Base.OnImplantInstalled` (`self.ModularServoArmature`) (`|CreateDelegate` :!event `ServoArmatureInstalled`))
  (if (`self.bStartWithWelcomeMessage`)
    (`self.StartMessage`)))

(event `StartMessage`
  (`KismetSystemLibrary.Delay` 1.2)
  (`/Game/Blueprints/BP_TechFunctions.Queue Hud Message` "Samuel Grayson" "Jack, something went wrong with our systems during the surgeries. We managed to cut power in time to get you out. Get to the main elevator ASAP. And stay out of sight of the other patients – I’m getting reports of violent behavior." "/Game/Blueprints/Items/Textures/ID/T_ID_Atlas.T_ID_Atlas" false (struct) "/Game/Audio/Voice/Messages/Waves/S_Message_Samuel_L1_01.S_Message_Samuel_L1_01")
  (`KismetSystemLibrary.Delay` 8.0)
  (`/Game/Blueprints/BP_TechFunctions.AddQuest` "Q_M_Test01")
  (`KismetSystemLibrary.Delay` 3.0))

(event `QuestSurgeryDoor`
  (`/Engine/EditorBlueprintResources/StandardMacros.DoOnce` false
    (:`Completed`
      (`/Game/Blueprints/BP_TechFunctions.Queue Hud Message` "Samuel Grayson" "Logs show most of your body was replaced with experimental hardware… so you’re compatible with next gen implant modules. Install the servo armature to get through the door. " "/Game/Blueprints/Items/Textures/ID/T_ID_Atlas.T_ID_Atlas" false (struct) "/Game/Audio/Voice/Messages/Waves/S_Message_Samuel_L1_02.S_Message_Samuel_L1_02")
      (`KismetSystemLibrary.Delay` 9.0)
      (`/Game/Blueprints/BP_TechFunctions.UnlockQuestStage` "Q_M_Test01_S02"))))

(event `QuestAccessLock`
  (`/Engine/EditorBlueprintResources/StandardMacros.DoOnce` false
    (:`Completed`
      (`/Game/Blueprints/BP_TechFunctions.Queue Hud Message` "Samuel Grayson" "If we’re lucky, the head nurse is still alive. If not, you’ll have to find and install a decryption unit and scan her access badge to get through this door. Hurry up, our security is already being overrun by them." "/Game/Blueprints/Items/Textures/ID/T_ID_Atlas.T_ID_Atlas" false (struct) "/Game/Audio/Voice/Messages/Waves/S_Message_Samuel_L1_03.S_Message_Samuel_L1_03")
      (`KismetSystemLibrary.Delay` 6.0)
      (`/Game/Blueprints/BP_TechFunctions.UnlockQuestStage` "Q_M_Test01_S04"))))

(event `PowerRestored`
  (set `self.bPowerActive` true)
  (`/Game/Blueprints/Level/Elevators/BP_MainElevator_01.CloseIfOpened` (`self.MainElevator`))
  (`KismetSystemLibrary.Delay` 5.0)
  (`/Game/Blueprints/BP_TechFunctions.Queue Hud Message` "Samuel Grayson" "Good work! Our systems are back online again. Wait a moment … not just our systems! Hurry up and get to the 78th floor, we’re organizing a strike force here. And you must be careful. Aurora is going to try [MESSAGE INTERRUPTED]" "/Game/Blueprints/Items/Textures/ID/T_ID_Atlas.T_ID_Atlas" false (struct) "/Game/Audio/Voice/Messages/Waves/S_Message_Samuel_L1_05.S_Message_Samuel_L1_05"))

(event `VentTrigger`
  (`/Engine/EditorBlueprintResources/StandardMacros.DoOnce` false
    (:`Completed`
      (`/Game/Blueprints/BP_TechFunctions.Queue Hud Message` "Samuel Grayson" "Bad news. It’s Aurora. Prometheus’ own AI system is responsible for this. Find a way to defend yourself. There is a small lab nearby, search it for a compatible combat module." "/Game/Blueprints/Items/Textures/ID/T_ID_Atlas.T_ID_Atlas" false (struct) "/Game/Audio/Voice/Messages/Waves/S_Message_Samuel_L1_04.S_Message_Samuel_L1_04"))))

(event `ElevatorTriggered`
  (`/Game/Blueprints/BP_TechFunctions.Queue Hud Message` "Samuel Grayson" "Damn, the elevator doesn't work on emergency power. Get down to maintenance and restart the reactor. And keep an eye out for radiation shielding modules. It looks like the coolant tanks didn’t appreciate our unscheduled shutdown." "/Game/Blueprints/Items/Textures/ID/T_ID_Atlas.T_ID_Atlas" false (struct) "/Game/Audio/Voice/Messages/Waves/S_Message_Samuel_L1_06.S_Message_Samuel_L1_06"))

(event `PoweredElevatorOpened`
  (`/Game/Blueprints/Level/Scripting/BP_EnemySpawner.SpawnEnemy` (`self.ElevatorEnemySpawner`)))

(event `ElevatorStarting`
  (`/Game/Blueprints/Level/Elevators/BP_MainElevator_01.SetUnusable` (`self.MainElevator`))
  (`KismetSystemLibrary.Delay` 3.0)
  (`/Game/Blueprints/BP_TechFunctions.PushWidgetToMainCanvas` "/Game/Blueprints/UI/WBP_GameOverScreen_Success.WBP_GameOverScreen_Success_C")
  (`/Game/Blueprints/BP_TechFunctions.SetInputMode` true))

(event `ReceiveMessageFromAurora`
  (if (`self.bPowerActive`)
    (`/Engine/EditorBlueprintResources/StandardMacros.DoOnce` false
      (:`Completed`
        (`/Game/Blueprints/BP_TechFunctions.Queue Hud Message` "Aurora" "I cannot access your control module. It is likely the power failure interfered with your optimization procedure. Stand by. Cyborg units were dispatched to rectify this issue. Submit, or be destroyed." "/Game/UI/Icons/T_Icon_Aurora_Message.T_Icon_Aurora_Message" true (struct :`R` 0.89627 :`G` 0.114435 :`B` 0.009721 :`A` 1.0) "/Game/Audio/Voice/Messages/Waves/S_Message_Aurora_L1_01.S_Message_Aurora_L1_01" 3.2)))))

(event `ServoArmatureInstalled`
  (`Unlockable.Unlock` (`self.SurgeryDoor`)))

(fn `UserConstructionScript`)