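; Level 01 scripted trigger that stages the first cyborg's introduction by killing a victim when the player overlaps it.
; A one-shot overlap plays the victim's crawl animation, then delays time the cyborg's dart sound and the hit.
; The shot is faked by spawning a dart, blood splat and impact sound at the head bone.
; The victim then ragdolls over a spawned blood pool, and the cyborg receives its patrol route.
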(event `self.ReceiveBeginPlay`)

(event `self.ReceiveActorBeginOverlap`
  (params (OtherActor :type "Actor Object Reference"))
  (if (== OtherActor (`GameplayStatics.GetPlayerCharacter` 0))
    (`/Engine/EditorBlueprintResources/StandardMacros.DoOnce` false
      (:`Completed`
        (`self.FirstCyborgIntroduction`)))))

(event `FirstCyborgIntroduction`
  (bind _skeletalmeshcomponent (`SkeletalMeshActor.SkeletalMeshComponent` (`self.VictimMesh`)))
  (bind _returnvalue (`SkinnedMeshComponent.GetBoneTransform` (`SkeletalMeshActor.SkeletalMeshComponent` (`self.VictimMesh`)) "head" "RTS_World"))
  (bind _returnvalue_2 (`SkinnedMeshComponent.GetBoneTransform` _skeletalmeshcomponent "head" "RTS_World"))
  (`SkeletalMeshComponent.PlayAnimation` _skeletalmeshcomponent "/Game/ThirdParty/DeathAnims/Deaths_Shoulder_Crawl.Deaths_Shoulder_Crawl" false)
  (`KismetSystemLibrary.Delay` 6.47)
  (`GameplayStatics.SpawnSoundAtLocation` "/Game/Audio/Weapons/Fire/MS_Weapon_Cyborg_Dart.MS_Weapon_Cyborg_Dart" (`self.K2_GetActorLocation` (`self.FirstCyborg`)) (struct) 1.0 1.0 0.0 null null)
  (`KismetSystemLibrary.Delay` 0.47)
  (`|SpawnActorFromClass` "/Game/Blueprints/Projectiles/BP_Projectile_Dart_CyborgLight.BP_Projectile_Dart_CyborgLight_C" _returnvalue_2 "AlwaysSpawn" "MultiplyWithRoot" null null)
  (`GameplayStatics.SpawnEmitterAtLocation` "/Game/ThirdParty/Realistic_Starter_VFX_Pack_Vol2/Particles/TechBreach/P_Blood_Splat_Spherical.P_Blood_Splat_Spherical" (.location _returnvalue_2) (.rotation _returnvalue_2) (.scale _returnvalue_2))
  (`GameplayStatics.SpawnSoundAttached` "/Game/Audio/Weapons/Impacts/MS_Hit_Flesh_Weakspot.MS_Hit_Flesh_Weakspot" _skeletalmeshcomponent "head" (0.0 0.0 0.0) (struct) "KeepRelativeOffset" false 1.0 1.0 0.0 null null)
  (`KismetSystemLibrary.Delay` 0.3)
  (`PrimitiveComponent.SetSimulatePhysics` _skeletalmeshcomponent true)
  (`|SpawnActorFromClass` "/Game/Blueprints/Level/Props/BP_BloodPool.BP_BloodPool_C" (`KismetMathLibrary.MakeTransform` (`KismetMathLibrary.MakeVector` (.x (.location _returnvalue)) (.y (.location _returnvalue)) 100.0)) "Undefined" "MultiplyWithRoot" null null)
  (set `/Game/Blueprints/Enemies/BP_Enemy_CyborgOperator_01.PatrolRoute` (`self.FirstCyborgPatrolRoute`) (`self.FirstCyborg`)))

(fn `UserConstructionScript`)