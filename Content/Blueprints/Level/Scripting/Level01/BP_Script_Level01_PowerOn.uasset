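; Level 01 scripting actor that reacts to power being restored at the reactor console.
; On BeginPlay it retries every tenth of a second until it finds the console, then binds to its power-restored event.
; The PowerOn event triggers the referenced enemy spawners, unhides listed actors and activates an audio component.
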(event `self.ReceiveBeginPlay`
  (bind _returnvalue (`GameplayStatics.GetActorOfClass` "/Game/Blueprints/Level/Interactable/BP_Interactable_ReactorConsole.BP_Interactable_ReactorConsole_C" :!label _label))
  (`/Engine/EditorBlueprintResources/StandardMacros.IsValid` _returnvalue
    (:`Is Valid`
      (add `/Game/Blueprints/Level/Interactable/BP_Interactable_ReactorConsole.OnPowerRestored` _returnvalue (`|CreateDelegate` :!event `PowerOn`)))
    (:`Is Not Valid`
      (`KismetSystemLibrary.Delay` 0.1)
      (goto _label))))

(event `PowerOn`
  (`|ExecutionSequence`
    (:`then_0`
      (for _array_element (`self.EnemySpawners`)
        (`/Game/Blueprints/Level/Scripting/BP_EnemySpawner.SpawnEnemy` _array_element)))
    (:`then_1`
      (for _array_element_2 (`self.ActorsToUnhide`)
        (`self.SetActorHiddenInGame` _array_element_2 false)))
    (:`then_2`
      (`ActorComponent.SetActive` (`AmbientSound.AudioComponent` (`self.AudioToActivate`)) true false))))

(fn `UserConstructionScript`)