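; Level 01 music trigger that gates its inherited trigger behavior on the level's power state.
; On BeginPlay it looks up the BP_Script_Level01_01 actor, retrying after a short delay until found, and caches it.
; When triggered, it calls the parent logic if TriggerWithPowerOn is set, otherwise only while the script actor's PowerActive is false.
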(event `self.ReceiveBeginPlay`
  (`parent.ReceiveBeginPlay`)
  (bind _returnvalue (`GameplayStatics.GetActorOfClass` "/Game/Blueprints/Level/Scripting/Level01/BP_Script_Level01_01.BP_Script_Level01_01_C" :!label _label))
  (`/Engine/EditorBlueprintResources/StandardMacros.IsValid` _returnvalue
    (:`Is Valid`
      (set `self.ScriptActor` _returnvalue))
    (:`Is Not Valid`
      (`KismetSystemLibrary.Delay` 0.1)
      (goto _label))))

(event `self.Triggered`
  (if (`self.bTriggerWithPowerOn`)
    (`parent.Triggered` :!label _label_2)
    (elif (not (`/Game/Blueprints/Level/Scripting/Level01/BP_Script_Level01_01.bPowerActive` (`self.ScriptActor`)))
      (goto _label_2))))

(fn `UserConstructionScript`
  (`parent.UserConstructionScript`))