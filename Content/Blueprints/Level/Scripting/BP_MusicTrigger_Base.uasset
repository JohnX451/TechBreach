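; BP_MusicTrigger_Base is a level trigger that starts a music track when the player pawn enters its box.
; On BeginPlay it looks up the BP_MusicManager actor, retrying after a short delay until it finds a valid one.
; A player overlap fires the Triggered event, gated by a DoOnce when TriggerOnce is set, which tells the manager to begin playing the trigger's Track.
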(event `self.ReceiveBeginPlay`
  (bind _returnvalue (`GameplayStatics.GetActorOfClass` "/Game/Blueprints/MusicSystem/BP_MusicManager.BP_MusicManager_C" :!label _label))
  (`/Engine/EditorBlueprintResources/StandardMacros.IsValid` _returnvalue
    (:`Is Valid`
      (set `self.MusicManager` _returnvalue))
    (:`Is Not Valid`
      (`KismetSystemLibrary.Delay` 0.1)
      (goto _label))))

(event `self.Box.OnComponentBeginOverlap`
  (params (OverlappedComponent :type "PrimitiveComponent Object Reference") (OtherActor :type "Actor Object Reference") (OtherComp :type "PrimitiveComponent Object Reference") (OtherBodyIndex :type Integer) (bFromSweep :type Boolean) (SweepResult :type "HitResult Structure (by ref)"))
  (if (== OtherActor (`GameplayStatics.GetPlayerPawn` 0))
    (if (`self.bTriggerOnce`)
      (`/Engine/EditorBlueprintResources/StandardMacros.DoOnce` false
        (:`Completed`
          _)))
    (`self.Triggered`)))

(event `Triggered`
  (`/Game/Blueprints/MusicSystem/BP_MusicManager.BeginPlayingTrack` (`self.MusicManager`) (`self.Track`)))

(fn `UserConstructionScript`)