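; Call console for a cargo lift, placed at the upper or lower stop as set by IsUp.
; Use triggers the linked Lift with that side and disables the console.
; Lift arrival events, bound shortly after BeginPlay, re-enable it only when the lift is at the opposite end.
; Active state is the "highlightable" component tag; disabling clears all tags on the Console component and turns off its custom-depth highlight.
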(event `self.ReceiveBeginPlay`
  (bind _lift (`self.Lift`))
  (`KismetSystemLibrary.Delay` 0.2)
  (add `/Game/Blueprints/Level/Elevators/BP_CargoLift.OnArriveDown` _lift (`|CreateDelegate` :!event `LiftArriveDown`))
  (add `/Game/Blueprints/Level/Elevators/BP_CargoLift.OnArriveUp` _lift (`|CreateDelegate` :!event `LiftArriveUp`))
  (if (== (`/Game/Blueprints/Level/Elevators/BP_CargoLift.bIsUp` _lift) (`self.bIsUp`))
    (`self.ChangeConsoleStatus` false)))

(event `self.Use`
  (`/Game/Blueprints/Level/Elevators/BP_CargoLift.TriggerLift` (`self.Lift`) (`self.bIsUp`))
  (`self.ChangeConsoleStatus` false))

(fn `ChangeConsoleStatus`
  (params (bSetActive :type Boolean))
  (bind _console (`self.Console`))
  (bind _componenttags (`ActorComponent.ComponentTags` _console))
  (if bSetActive
    (`KismetArrayLibrary.Array_Add` _componenttags "highlightable")
    (else
      (`PrimitiveComponent.SetRenderCustomDepth` _console false)
      (`KismetArrayLibrary.Array_Clear` _componenttags))))

(fn `LiftArriveDown`
  (`self.ChangeConsoleStatus` (`self.bIsUp`)))

(fn `LiftArriveUp`
  (`self.ChangeConsoleStatus` (not (`self.bIsUp`))))

(fn `UserConstructionScript`)