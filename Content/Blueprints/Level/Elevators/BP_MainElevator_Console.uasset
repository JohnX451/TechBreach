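; Interactable console for the main elevator that starts the ride when powered and reports an error when main power is offline.
; A popup widget shows the use prompt, and Use branches on HasPower, with one-shot logic on each path driving the info text, quest component and event dispatchers.
; The powered path also locks the elevator, removes the prompt and highlight, and plays a delayed start sound.
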(event `self.ReceiveBeginPlay`
  (bind _aswbp_hud_popup_simple (cast `/Game/Blueprints/UI/HUD/WBP_HUD_Popup_Simple` (`WidgetComponent.GetWidget` (`self.Widget`))))
  (`/Game/Blueprints/UI/HUD/WBP_HUD_Popup_Simple.SetText` _aswbp_hud_popup_simple "USE MAIN ELEVATOR"))

(event `self.SetInteractionPopup`
  (params (bShow :type Boolean))
  (bind _widget (`self.Widget`)
    (:`then`
      (`SceneComponent.SetHiddenInGame` _widget (not bShow) false))
    (:`else`)))

(event `self.Use`
  (bind _bp_questactorcomponent (`self.BP_QuestActorComponent`))
  (if (`self.bHasPower`)
    (`/Engine/EditorBlueprintResources/StandardMacros.DoOnce` false
      (:`Completed`
        (`/Game/Blueprints/Level/Elevators/BP_MainElevator_01.SetUnusable` (`self.MainElevator`))
        (`TextRenderComponent.K2_SetText` (`self.InfoText`) "Level B02 \n \nMoving... \n Next: B01")
        (`/Game/Blueprints/QuestSystem/AC_QuestActorComponent.QuestInteraction` (`self.BP_QuestActorComponent`))
        (`PrimitiveComponent.SetRenderCustomDepth` (`self.StaticMesh`) false)
        (`ActorComponent.K2_DestroyComponent` (`self.Widget`))
        (`self.OnElevatorStarting`)
        (`KismetSystemLibrary.Delay` 3.1)
        (`GameplayStatics.PlaySound2D` "/Game/Audio/Misc/MS_Prop_MainElevator_Start.MS_Prop_MainElevator_Start" 1.2 1.0 0.0 null null)))
    (else
      (`/Game/Blueprints/BP_TechFunctions.ShowHint` "Main power offline.")
      (`/Engine/EditorBlueprintResources/StandardMacros.DoOnce` false
        (:`Completed`
          (`TextRenderComponent.K2_SetText` (`self.InfoText`) "Level B02 \n \nError: \n  main power offline \n  [E-04562]")
          (`/Game/Blueprints/QuestSystem/AC_QuestActorComponent.QuestInteraction` _bp_questactorcomponent)
          (`/Game/Blueprints/QuestSystem/AC_QuestActorComponent.UpdateDataForNextInteraction` _bp_questactorcomponent "NewEnumerator2" "Q_M_Test01_S01_O01")
          (`self.OnActivatedNoPower`))))))

(fn `UserConstructionScript`)