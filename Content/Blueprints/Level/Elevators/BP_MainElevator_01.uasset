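; BP_MainElevator_01 is an elevator Blueprint whose inner and outer main doors swing open and closed on use.
; Use ignores input while busy, otherwise passes the closed state to ChangeDoorState to toggle the doors.
; The MoveDoors timeline plays forward or in reverse, yawing the two door meshes in opposite directions.
; When opening or closing finishes, it updates DoorsClosed and clears the busy flag.
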(event `self.Use`
  (if (not (`self.bIsBusy`))
    (`self.ChangeDoorState` (`self.bDoorsClosed`))))

(event `ChangeDoorState`
  (params (bOpen :type Boolean))
  (set `self.bIsBusy` true)
  (if bOpen
    (bind (_direction _rotationz) (`Timeline|MoveDoors` :!via `PlayFromStart` :!label _label)
      (:`Update`
        (`SceneComponent.K2_SetRelativeRotation` (`self.SM_ElevatorMainDoorOuter_01`) (`KismetMathLibrary.MakeRotator` 0.0 0.0 (* _rotationz 73.0)) false false)
        (`SceneComponent.K2_SetRelativeRotation` (`self.SM_ElevatorMainDoorInner_01`) (`KismetMathLibrary.MakeRotator` 0.0 0.0 (* _rotationz -73.0)) false false))
      (:`Finished`
        (set `self.bDoorsClosed` (not bOpen))
        (set `self.bIsBusy` false)))
    (else
      (goto _label :!via `ReverseFromEnd`))))

(fn `UserConstructionScript`)