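; BP_CargoLift is a cargo lift that toggles between a lower and raised position when used or triggered.
; A timeline, played forward or reversed, moves the root vertically by Height from the position captured in the construction script, which also applies the IsUp start state.
; During travel it ignores triggers and strips the console's tags and custom-depth highlight, then restores the "highlightable" tag and calls arrival events.
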(event `self.ReceiveBeginPlay`)

(event `self.Use`
  (`self.TriggerLift` (not (`self.bIsUp`))))

(event `TriggerLift`
  (params (bGoUp :type Boolean))
  (if (not (`self.bIsMoving`))
    (if (!= bGoUp (`self.bIsUp`))
      (`self.MoveLift` bGoUp)
      (`self.ChangeConsoleStatus` false))))

(event `MoveLift`
  (params (bDirectionUp :type Boolean))
  (bind _defaultsceneroot (`self.DefaultSceneRoot`))
  (bind (_initialposition_x _initialposition_y _initialposition_z) (`KismetMathLibrary.BreakVector` (`self.InitialPosition`)))
  (bind (_returnvalue_x _returnvalue_y) (`KismetMathLibrary.BreakVector` (`SceneComponent.K2_GetComponentLocation` _defaultsceneroot)))
  (set `self.bIsMoving` true)
  (if bDirectionUp
    (bind (_direction _liftheight) (`Timeline|LiftTimeline` :!via `PlayFromStart` :!label _label)
      (:`Update`
        (`SceneComponent.K2_SetWorldLocation` _defaultsceneroot (`KismetMathLibrary.MakeVector` _returnvalue_x _returnvalue_y (+ (* _liftheight (`self.Height`)) _initialposition_z)) false false))
      (:`Finished`
        (set `self.bIsMoving` false)
        (`self.ChangeConsoleStatus` true)
        (bind _output_get (set `self.bIsUp` (not (`self.bIsUp`))))
        (if _output_get
          (`self.OnArriveUp`)
          (else
            (`self.OnArriveDown`)))))
    (else
      (goto _label :!via `ReverseFromEnd`))))

(fn `ChangeConsoleStatus`
  (params (bSetActive :type Boolean))
  (bind _console (`self.Console`))
  (bind _componenttags (`ActorComponent.ComponentTags` _console))
  (if bSetActive
    (`KismetArrayLibrary.Array_Add` _componenttags "highlightable")
    (else
      (`PrimitiveComponent.SetRenderCustomDepth` _console false)
      (`KismetArrayLibrary.Array_Clear` _componenttags))))

(fn `UserConstructionScript`
  (bind (_initialposition_x _initialposition_y _initialposition_z) (`KismetMathLibrary.BreakVector` (`self.InitialPosition`)))
  (set `self.InitialPosition` (`SceneComponent.K2_GetComponentLocation` (`self.DefaultSceneRoot`)))
  (if (`self.bIsUp`)
    (`SceneComponent.K2_SetWorldLocation` (`self.DefaultSceneRoot`) (`KismetMathLibrary.MakeVector` _initialposition_x _initialposition_y (+ _initialposition_z (`self.Height`))) false false)))