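; Spawner actor that plays impact VFX and sound at a hit location on BeginPlay, based on surface type, damage and weakspot flag.
; InitializeValues maps hit damage to clamped effect count and uniform scale, doubling both for weakspot hits.
; HandleVFX spawns a blood or metal Niagara system along the hit normal, setting its spawn multiplier before activation.
; HandleSFX plays a flesh or armor sound, with separate weakspot variants.
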(event `self.ReceiveBeginPlay`
  (`self.InitializeValues`)
  (`self.HandleVFX`)
  (`self.HandleSFX`))

(fn `HandleSFX`
  (locals (HitSFX :type "SoundBase Object Reference"))
  (bind _surfacetype (`self.SurfaceType`))
  (if (`self.bHitWeakspot`)
    (set `local.HitSFX` (select `int` _surfacetype :`0` "/Game/Audio/Weapons/Impacts/MS_Hit_Flesh_Weakspot.MS_Hit_Flesh_Weakspot" :`1` "/Game/Audio/Weapons/Impacts/MS_Hit_Armor_Weakspot.MS_Hit_Armor_Weakspot" :!type "SoundBase Object Reference"))
    (else
      (set `local.HitSFX` (select `int` _surfacetype :`0` "/Game/Audio/Weapons/Impacts/MS_Hit_Flesh.MS_Hit_Flesh" :`1` "/Game/Audio/Weapons/Impacts/MS_Hit_Armor.MS_Hit_Armor" :!type "SoundBase Object Reference"))))
  (`GameplayStatics.PlaySoundAtLocation` (`local.HitSFX`) (`self.HitLocation`) (struct) 1.0 1.0 0.0 null null null null))

(fn `HandleVFX`
  (bind _returnvalue (`NiagaraFunctionLibrary.SpawnSystemAtLocation` (select `int` (`self.SurfaceType`) :`0` "/Game/ThirdParty/BallisticsVFX/Particles/Impacts/DynamicImpacts/TechBreach/NS_Impact_Blood.NS_Impact_Blood" :`1` "/Game/ThirdParty/BallisticsVFX/Particles/Impacts/DynamicImpacts/TechBreach/NS_Impact_Metal.NS_Impact_Metal" :!type "NiagaraSystem Object Reference") (`self.HitLocation`) (`KismetMathLibrary.MakeRotFromZ` (`self.HitNormal`)) (`self.EffectScale`) true false))
  (`NiagaraComponent.SetVariableInt` _returnvalue "SpawnMultiplierPercentage" (`self.EffectCount`))
  (`ActorComponent.Activate` _returnvalue false))

(fn `InitializeValues`
  (bind _returnvalue (* (`KismetMathLibrary.MapRangeClamped` (`self.HitDamage`) 10.0 50.0 0.2 0.5) (`KismetMathLibrary.SelectFloat` 2.0 1.0 (`self.bHitWeakspot`))))
  (set `self.EffectCount` (* (`KismetMathLibrary.Round` (`KismetMathLibrary.MapRangeClamped` (`self.HitDamage`) 10.0 50.0 5.0 50.0)) (`KismetMathLibrary.SelectInt` 2 1 (`self.bHitWeakspot`))))
  (set `self.EffectScale` (`KismetMathLibrary.MakeVector` _returnvalue _returnvalue _returnvalue)))

(fn `UserConstructionScript`)