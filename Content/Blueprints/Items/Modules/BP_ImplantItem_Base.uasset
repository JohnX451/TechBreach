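; Base Blueprint for world implant items that open the implant installation menu when used, passing in their Implant module.
; The interaction popup toggles the widget's visibility and fills its WBP_HUD_Popup_Stats with the implant's stats.
; The construction script derives the item's look from the Implant, setting the label to its display name and applying its UI image through a dynamic material instance on the mesh.
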(event `self.Use`
  (`/Game/Blueprints/BP_TechFunctions.ShowImplantInstallationMenu` (`self.Implant`) self))

(event `self.SetInteractionPopup`
  (params (bShow :type Boolean))
  (bind _widget (`self.Widget`))
  (`SceneComponent.SetHiddenInGame` _widget (not bShow) false)
  ;[1 1 1] Show Stats if any
  (bind _aswbp_hud_popup_stats (cast `/Game/Blueprints/UI/HUD/WBP_HUD_Popup_Stats` (`WidgetComponent.GetUserWidgetObject` _widget)))
  (`/Game/Blueprints/UI/HUD/WBP_HUD_Popup_Stats.Setup` :`self` _aswbp_hud_popup_stats :`Module` (`self.Implant`)))

(fn `UserConstructionScript`
  (bind (_implant_attributecoefterms _implant_installedsubmodules _implant_implantmesh _implant_imageui _implant_id _implant_displayname) (break `ImplantData` (`self.Implant`)))
  (`parent.UserConstructionScript`)
  (`TextRenderComponent.K2_SetText` (`self.Label`) (`KismetTextLibrary.Conv_NameToText` _implant_displayname))
  (bind _returnvalue (`PrimitiveComponent.CreateDynamicMaterialInstance` (`self.Mesh`) 0 "/Game/Materials/Items/MI_Image_Container.MI_Image_Container" "None"))
  (`MaterialInstanceDynamic.SetTextureParameterValue` _returnvalue "Image" _implant_imageui))