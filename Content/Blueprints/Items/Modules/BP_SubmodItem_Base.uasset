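; Base Blueprint for a world item that represents a submodule and lets it be installed through a menu.
; Its construction script sets the label to the submodule's display name and puts its UI image on the mesh through a dynamic material instance.
; Using the item opens the submodule installation menu with its submodule and itself as the caller, and the interaction popup event toggles the widget's visibility.
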(event `self.Use`
  (`/Game/Blueprints/BP_TechFunctions.ShowSubmodInstallationMenu` (`self.Submodule`) self))

(event `self.SetInteractionPopup`
  (params (bShow :type Boolean))
  (`SceneComponent.SetHiddenInGame` (`self.Widget`) (not bShow) false))

(fn `UserConstructionScript`
  (bind (_submodule_weapondata _submodule_attributecoefterms _submodule_compatibleimplantids _submodule_imageui _submodule_id _submodule_displayname) (break `SubmoduleData` (`self.Submodule`)))
  (`parent.UserConstructionScript`)
  (`TextRenderComponent.K2_SetText` (`self.Label`) (`KismetTextLibrary.Conv_NameToText` _submodule_displayname))
  (bind _returnvalue (`PrimitiveComponent.CreateDynamicMaterialInstance` (`self.Mesh`) 1 "/Game/Materials/Items/MI_Image_Container.MI_Image_Container" "None"))
  (`MaterialInstanceDynamic.SetTextureParameterValue` _returnvalue "Image" _submodule_imageui))