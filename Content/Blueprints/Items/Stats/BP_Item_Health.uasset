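; BP_Item_Health is an interactable health pickup that restores the player's health when used.
; On begin play it sets its widget prompt to "Press E to use", and SetInteractionPopup shows or hides that widget.
; Use adds RestoreHealth through player 0's BP_StatsComponent, then destroys the actor.
; The construction script writes the restore amount into a TextRender label.
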(event `self.ReceiveBeginPlay`
  (bind _aswbp_interact_01 (cast `/Game/Blueprints/Demo/UIDemo/WBP_Interact_01` (`WidgetComponent.GetWidget` (`self.Widget`))))
  (set `TextBlock.Text` "Press \"E\" to use" (`/Game/Blueprints/Demo/UIDemo/WBP_Interact_01.TextBlock_0` _aswbp_interact_01)))

(event `self.Use`
  (`StatsComponent.AddHealth` (`self.GetComponentByClass` (`GameplayStatics.GetPlayerCharacter` 0) "/Game/Blueprints/Components/BP_StatsComponent.BP_StatsComponent_C") (`self.RestoreHealth`))
  (`self.K2_DestroyActor`))

(event `self.SetInteractionPopup`
  (params (bShow :type Boolean))
  (`SceneComponent.SetHiddenInGame` (`self.Widget`) (not bShow) false))

(fn `UserConstructionScript`
  (`TextRenderComponent.K2_SetText` (`self.TextRender`) (`|FormatText` "Health: + {1}" (`self.RestoreHealth`))))