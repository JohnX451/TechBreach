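; BP_Item_Energy is an interactable pickup that restores the player's energy when used.
; On BeginPlay it sets its WBP_Interact_01 widget prompt to a recharge message, and SetInteractionPopup shows or hides that widget.
; Use adds RestoreEnergy to the player character's BP_StatsComponent, plays a battery sound, then destroys the item.
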(event `self.ReceiveBeginPlay`
  (bind _aswbp_interact_01 (cast `/Game/Blueprints/Demo/UIDemo/WBP_Interact_01` (`WidgetComponent.GetWidget` (`self.Widget`))))
  (set `TextBlock.Text` "Press \"E\" to recharge energy" (`/Game/Blueprints/Demo/UIDemo/WBP_Interact_01.CommonTextBlock_0` _aswbp_interact_01)))

(event `self.Use`
  (`StatsComponent.AddEnergy` (`self.GetComponentByClass` (`GameplayStatics.GetPlayerCharacter` 0) "/Game/Blueprints/Components/BP_StatsComponent.BP_StatsComponent_C") (`self.RestoreEnergy`))
  (`GameplayStatics.PlaySound2D` "/Game/Audio/Items/MS_Prop_Battery_01.MS_Prop_Battery_01" 1.0 1.0 0.0 null null)
  (`self.K2_DestroyActor`))

(event `self.SetInteractionPopup`
  (params (bShow :type Boolean))
  (`SceneComponent.SetHiddenInGame` (`self.Widget`) (not bShow) false))

(fn `UserConstructionScript`)