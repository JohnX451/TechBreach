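; BP_AccessCodeItem is an interactable item that grants the player its AccessCode once when used.
; Use passes the code to the player's AbilityComponent; on success it clears mesh tags and custom-depth highlight, hides the widget and starts the HUD scan progress.
; The interaction popup can show only while the item is unscanned and the player's access-code ability is active.
; The construction script writes the code into the item's label.
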(event `self.Use`
  (bind _sm_demo_item_02 (`self.SM_Demo_Item_02`))
  (if (not (`self.bWasScanned`))
    (bind _asbp_player_character (cast `/Game/Blueprints/Player/BP_PlayerCharacter` (`GameplayStatics.GetPlayerCharacter` 0))
      (:`then`
        (bind _returnvalue (`AbilityComponent.AddAccessCode` (`PlayerBaseCharacter.AbilityComponent` _asbp_player_character) (`self.AccessCode`)))
        (if _returnvalue
          (`KismetSystemLibrary.PrintText` (`|FormatText` "Adding AccessCode {AccessCode}" (`self.AccessCode`)))
          (`KismetArrayLibrary.Array_Clear` (`ActorComponent.ComponentTags` (`self.Mesh`)))
          (`KismetArrayLibrary.Array_Clear` (`ActorComponent.ComponentTags` _sm_demo_item_02))
          (`PrimitiveComponent.SetRenderCustomDepth` _sm_demo_item_02 false)
          (`PrimitiveComponent.SetRenderCustomDepth` (`self.Mesh`) false)
          (`SceneComponent.SetHiddenInGame` (`self.Widget`) true false)
          (set `self.bWasScanned` true)
          (`/Game/Blueprints/Demo/UIDemo/WBP_Demo_AccessCodeScanProgress.StartScanning` (`/Game/Blueprints/Demo/UIDemo/WBP_Demo_HUD.ScanProgress` (`/Game/Blueprints/Components/BP_StatsComponent.PlayerHUD` (`self.GetComponentByClass` (`GameplayStatics.GetPlayerCharacter` 0) "/Game/Blueprints/Components/BP_StatsComponent.BP_StatsComponent_C"))))
          (else
            (`KismetSystemLibrary.PrintString` "AccessCode could not be added"))))
      (:`CastFailed`
        (`KismetSystemLibrary.PrintString` "Player Cast Failed" :!label _label)))))

(event `self.SetInteractionPopup`
  (params (bShow :type Boolean))
  (bind _widget (`self.Widget`))
  (if (not (`self.bWasScanned`))
    (bind _asbp_player_character (cast `/Game/Blueprints/Player/BP_PlayerCharacter` (`GameplayStatics.GetPlayerCharacter` 0))
      (:`then`
        (bind _isaccesscodeabilityactive (`AbilityComponent.IsAccessCodeAbilityActive` (`PlayerBaseCharacter.AbilityComponent` _asbp_player_character)))
        (if _isaccesscodeabilityactive
          (`SceneComponent.SetHiddenInGame` _widget (not bShow) false)
          (else
            (`SceneComponent.SetHiddenInGame` _widget (not _isaccesscodeabilityactive) false))))
      (:`CastFailed`
        (goto _label)))))

(fn `UserConstructionScript`
  (`parent.UserConstructionScript`)
  (`TextRenderComponent.K2_SetText` (`self.Label`) (`|FormatText` "AccessCode {Code}" (`self.AccessCode`))))