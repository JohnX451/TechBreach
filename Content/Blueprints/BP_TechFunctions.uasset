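; BP_TechFunctions is a Blueprint function library of game-wide helpers for settings, HUD, module installation and quests.
; Audio and gameplay settings persist in SaveGame slots and are applied to a sound mix, the game instance and the player's mouse controls.
; UI helpers cast player 0's character to reach its HUD and widget canvas, pushing install, scan, hack, hint and message widgets.
; Other helpers wrap player components for quests and implants, and build menu list models.
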(fn `AddQuest`
  (params (QuestId :type Name))
  (`/Game/Blueprints/QuestSystem/AC_QuestLogComponent.AddQuest` (`Actor.GetComponentByClass` (`GameplayStatics.GetPlayerCharacter` (`local.__WorldContext`)) "/Game/Blueprints/QuestSystem/AC_QuestLogComponent.AC_QuestLogComponent_C") QuestId))

(fn `ApplyAudioSettings`
  (params (WorldContextObject :type "Object Object Reference"))
  (`GameplayStatics.SetBaseSoundMix` WorldContextObject "/Game/Audio/SoundMixMain.SoundMixMain")
  (bind (_bexists _audiosettings) (`self.LoadAudioSettings` WorldContextObject))
  (if _bexists
    (for _array_element _audiosettings
      (bind (_soundclass _volume) (break `/Game/Blueprints/UI/F_AudioSetting` _array_element))
      (`GameplayStatics.SetSoundMixClassOverride` (`local.__WorldContext`) "/Game/Audio/SoundMixMain.SoundMixMain" _soundclass _volume 1.0 0.0))))

(fn `ApplyGameplaySettings`
  (params (WorldContextObject :type "Object Object Reference"))
  (locals (GameInst :type "TechGameInstance Object Reference"))
  (bind _gameinst (`local.GameInst`))
  (bind (_gameplayoptions_healthcoefplayer _gameplayoptions_healthcoefenemy _gameplayoptions_mousesensitivity _gameplayoptions_mouseysign) (break `GameplayOptions` (`TechGameInstance.GameplayOptions` _gameinst)))
  (bind _gameplayoptions (`TechGameInstance.GameplayOptions` _gameinst))
  (bind (_bexists _gameplaysettings) (`self.LoadGameplaySettings` WorldContextObject))
  (if _bexists
    (bind _astech_game_instance (cast `TechGameInstance` (`GameplayStatics.GetGameInstance` WorldContextObject)))
    (set `local.GameInst` _astech_game_instance)
    (for _array_element _gameplaysettings
      (bind (_name _valuefloat _valuebool) (break `/Game/Blueprints/UI/F_GameplaySetting` _array_element))
      (switch `/Game/Blueprints/UI/E_GameplayOption` _name
        (:`NewEnumerator0`
          (bind _structout (setmembers `GameplayOptions` :`StructRef` _gameplayoptions :`HealthCoefPlayer` _valuefloat))
          (set `TechGameInstance.GameplayOptions` _structout _gameinst))
        (:`NewEnumerator1`
          (bind _structout_2 (setmembers `GameplayOptions` :`StructRef` _gameplayoptions :`HealthCoefEnemy` _valuefloat))
          (set `TechGameInstance.GameplayOptions` _structout_2 _gameinst))
        (:`NewEnumerator2`
          (bind _structout_3 (setmembers `GameplayOptions` :`StructRef` _gameplayoptions :`MouseSensitivity` _valuefloat))
          (set `TechGameInstance.GameplayOptions` _structout_3 _gameinst))
        (:`NewEnumerator3`
          (bind _structout_4 (setmembers `GameplayOptions` :`StructRef` _gameplayoptions :`MouseYSign` _valuefloat))
          (set `TechGameInstance.GameplayOptions` _structout_4 _gameinst))
        (:`NewEnumerator4`
          (bind _structout_5 (setmembers `GameplayOptions` :`StructRef` _gameplayoptions :`ShowSubtitles` _valuebool))
          (set `TechGameInstance.GameplayOptions` _structout_5 _gameinst))))
    (bind _asplayer_base_character (cast `PlayerBaseCharacter` (`GameplayStatics.GetPlayerCharacter` WorldContextObject)))
    (set `PlayerBaseCharacter.MouseSensitivity` _gameplayoptions_mousesensitivity _asplayer_base_character)
    (set `PlayerBaseCharacter.MouseYSign` _gameplayoptions_mouseysign _asplayer_base_character)
    (return)))

(fn `BeginAccessCodeScan`
  (params (CardID :type Name))
  (bind _commonactivatablewidget (`self.GetPlayerActiveHudWidget` (`local.__WorldContext`)))
  (bind _aswbp_hud_base (cast `/Game/Blueprints/UI/HUD/WBP_HUD_Base` _commonactivatablewidget))
  (bind _containercenter (`/Game/Blueprints/UI/HUD/WBP_HUD_Base.ContainerCenter` _aswbp_hud_base))
  (`/Engine/EditorBlueprintResources/StandardMacros.IsValid` _containercenter
    (:`Is Valid`
      (`/Game/Blueprints/UI/CommonUI/WBP_UserbaseCanvas.PushWidget` _containercenter "/Game/Blueprints/UI/HUD/WBP_HUD_AccessCode_Scan.WBP_HUD_AccessCode_Scan_C")
      (bind _commonactivatablewidget_2 (`/Game/Blueprints/UI/CommonUI/WBP_UserbaseCanvas.GetActiveWidget` _containercenter))
      (bind _aswbp_hud_access_code_scan (cast `/Game/Blueprints/UI/HUD/WBP_HUD_AccessCode_Scan` _commonactivatablewidget_2))
      (`/Game/Blueprints/UI/HUD/WBP_HUD_AccessCode_Scan.StartScanning` _aswbp_hud_access_code_scan (`local.CardID`)))))

(fn `BeginHack`
  (params (HackDuration :type "Float (double-precision)") (SystemName :type Name) (HackingLevel :type "EHackingLevel Enum" :default "None"))
  (bind _commonactivatablewidget (`self.GetPlayerActiveHudWidget` (`local.__WorldContext`)))
  (bind _aswbp_hud_base (cast `/Game/Blueprints/UI/HUD/WBP_HUD_Base` _commonactivatablewidget))
  (bind _containercenter (`/Game/Blueprints/UI/HUD/WBP_HUD_Base.ContainerCenter` _aswbp_hud_base))
  (`/Engine/EditorBlueprintResources/StandardMacros.IsValid` _containercenter
    (:`Is Valid`
      (`/Game/Blueprints/UI/CommonUI/WBP_UserbaseCanvas.PushWidget` _containercenter "/Game/Blueprints/UI/HUD/WBP_HUD_Hacking.WBP_HUD_Hacking_C")
      (bind _commonactivatablewidget_2 (`/Game/Blueprints/UI/CommonUI/WBP_UserbaseCanvas.GetActiveWidget` _containercenter))
      (bind _aswbp_hud_hacking (cast `/Game/Blueprints/UI/HUD/WBP_HUD_Hacking` _commonactivatablewidget_2))
      (`/Game/Blueprints/UI/HUD/WBP_HUD_Hacking.StartHacking` _aswbp_hud_hacking (`local.HackDuration`) (`local.SystemName`) (`local.HackingLevel`)))))

(fn `BeginModuleInstallation`
  (params (ImplantData :type "ImplantData Structure") (SubmoduleData :type "SubmoduleData Structure") (bIsSubmodule :type Boolean) (bReplaceOld :type Boolean) (bInstalledFromMenu :type Boolean) (ImplantSlot :type "EImplantSlot Enum" :default "Head1") (NewIndex :type Integer))
  (`self.SetInputMode` true null false (`local.__WorldContext`))
  (bind _commonactivatablewidget (`self.GetPlayerActiveHudWidget` (`local.__WorldContext`)))
  (bind _aswbp_hud_base (cast `/Game/Blueprints/UI/HUD/WBP_HUD_Base` _commonactivatablewidget)
    (:`then`
      (bind _containercenter (`/Game/Blueprints/UI/HUD/WBP_HUD_Base.ContainerCenter` _aswbp_hud_base))
      (`/Engine/EditorBlueprintResources/StandardMacros.IsValid` _containercenter
        (:`Is Valid`
          (`/Game/Blueprints/UI/CommonUI/WBP_UserbaseCanvas.PushWidget` _containercenter "/Game/Blueprints/UI/HUD/WBP_InstallProgress.WBP_InstallProgress_C")
          (bind _commonactivatablewidget_2 (`/Game/Blueprints/UI/CommonUI/WBP_UserbaseCanvas.GetActiveWidget` _containercenter))
          (bind _aswbp_install_progress (cast `/Game/Blueprints/UI/HUD/WBP_InstallProgress` _commonactivatablewidget_2)
            (:`then`
              (`/Game/Blueprints/UI/HUD/WBP_InstallProgress.StartInstallation` _aswbp_install_progress (`local.ImplantData`) (`local.SubmoduleData`) (`local.bIsSubmodule`) (`local.ImplantSlot`) (`local.NewIndex`) (`local.bReplaceOld`) (`local.bInstalledFromMenu`)))
            (:`CastFailed`
              (`KismetSystemLibrary.PrintString` (`local.__WorldContext`) "Begin Module Installation: Install Progress Widget not casted correctly"))))
        (:`Is Not Valid`
          (`KismetSystemLibrary.PrintString` (`local.__WorldContext`) "Begin Module Installation: Progress Bar Container not valid"))))
    (:`CastFailed`
      (`KismetSystemLibrary.PrintString` (`local.__WorldContext`) "Begin Module Installation: Cast to HUD Base failed"))))

(fn `CompleteObjective`
  (params (ObjectiveId :type Name))
  (`/Game/Blueprints/QuestSystem/AC_QuestLogComponent.CompleteObjective` (`Actor.GetComponentByClass` (`GameplayStatics.GetPlayerCharacter` (`local.__WorldContext`)) "/Game/Blueprints/QuestSystem/AC_QuestLogComponent.AC_QuestLogComponent_C") ObjectiveId))

(fn `GetImplantStatsFormatted`
  (params (ImplantData :type "ImplantData Structure"))
  (returns (ImplantStatsFormatted :type Text))
  (locals (Output :type Text) (AttributeTypes :type "Array of EAttributeType Enum"))
  (for _array_element (`local.AttributeTypes`)
    (bind _value (`BlueprintMapLibrary.Map_Find` ImplantData_AttributeCoefTerms _array_element))
    (if (!= _value 0.0)
      (if (`KismetTextLibrary.TextIsEmpty` (`local.Output`))
        (bind _returnvalue (`|GetEnumeratorNameAsString` _array_element))
        (bind _returnvalue_2 (`KismetTextLibrary.Conv_DoubleToText` _value "HalfToEven" true true 1 324 2 2))
        (set `local.Output` (`|FormatText` "{attribute}: {value}" _returnvalue _returnvalue_2))
        (else
          (set `local.Output` (`|FormatText` "{before} \n{attribute}: {value}" (`local.Output`) _returnvalue _returnvalue_2))))))
  (return (`local.Output`)))

(fn `GetModelImplants`
  (params (OwningWidget :type "Widget Object Reference"))
  (returns (Output1 :type "Array of /Game/Blueprints/BP_Implant_Model Object Reference"))
  (locals (Output :type "Array of /Game/Blueprints/BP_Implant_Model Object Reference") (Slots :type "Array of EImplantSlot Enum"))
  (bind _owningwidget (`local.OwningWidget`))
  (bind _returnvalue (`Actor.GetComponentByClass` (`GameplayStatics.GetPlayerCharacter` (`local.__WorldContext`)) "/Script/TechBreach.ModulesComponent"))
  (`|ExecutionSequence`
    (:`then_0`
      (for _array_element (`ModulesComponent.InactiveImplants` _returnvalue)
        (bind _returnvalue_2 (`|GenericCreateObject` _owningwidget "/Game/Blueprints/BP_Implant_Model.BP_Implant_Model_C" (make `/Game/Blueprints/F_Implant` _array_element) false))
        (`KismetArrayLibrary.Array_Add` (`local.Output`) _returnvalue_2)))
    (:`then_1`
      (for _array_element_2 (`local.Slots`)
        (bind (_value _returnvalue_3) (`BlueprintMapLibrary.Map_Find` (`ModulesComponent.ActiveImplants` _returnvalue) _array_element_2))
        (if _returnvalue_3
          (bind _returnvalue_4 (`|GenericCreateObject` _owningwidget "/Game/Blueprints/BP_Implant_Model.BP_Implant_Model_C" (make `/Game/Blueprints/F_Implant` _value _array_element_2) true))
          (`KismetArrayLibrary.Array_Add` (`local.Output`) _returnvalue_4)))
      (return (`local.Output`)))))

(fn `GetModelPlayerStats`
  (params (OwningWidget :type "Widget Object Reference"))
  (returns (PlayerStatObjects :type "Array of /Game/Blueprints/BP_Stats_Model Object Reference"))
  (locals (ListModelArray :type "Array of /Game/Blueprints/BP_Stats_Model Object Reference"))
  (bind _returnvalue (`GameplayStatics.GetPlayerCharacter` (`local.__WorldContext`)))
  (bind _returnvalue_2 (`Actor.GetComponentByClass` _returnvalue "/Script/TechBreach.AbilityComponent"))
  (bind _currentattributevalues (`StatsComponent.CurrentAttributeValues` (`Actor.GetComponentByClass` _returnvalue "/Script/TechBreach.StatsComponent")))
  (bind _keys (`BlueprintMapLibrary.Map_Keys` _currentattributevalues))
  (for _array_element _keys
    (bind _returnvalue_3 (`|GenericCreateObject` (`local.OwningWidget`) "/Game/Blueprints/BP_Stats_Model.BP_Stats_Model_C" (`KismetTextLibrary.Conv_StringToText` (`|GetEnumeratorNameAsString` _array_element)) (`KismetTextLibrary.Conv_DoubleToText` (`BlueprintMapLibrary.Map_Find` _currentattributevalues _array_element) "HalfToEven" false true 1 324 0 2)))
    (`KismetArrayLibrary.Array_Add` (`local.ListModelArray`) _returnvalue_3))
  (bind _returnvalue_4 (`|GenericCreateObject` (`local.OwningWidget`) "/Game/Blueprints/BP_Stats_Model.BP_Stats_Model_C" "Can use access badges" (select `bool` (`AbilityComponent.IsAccessCodeAbilityActive` _returnvalue_2) :`false` "No" :`true` "Yes" :!type "Text")))
  (`KismetArrayLibrary.Array_Add` (`local.ListModelArray`) _returnvalue_4)
  (bind _returnvalue_5 (`|GenericCreateObject` (`local.OwningWidget`) "/Game/Blueprints/BP_Stats_Model.BP_Stats_Model_C" "Hacking level" (`KismetTextLibrary.Conv_StringToText` (`|GetEnumeratorNameAsString` (`AbilityComponent.HackingLevel` _returnvalue_2)))))
  (`KismetArrayLibrary.Array_Add` (`local.ListModelArray`) _returnvalue_5)
  (return (`local.ListModelArray`)))

(fn `GetModelSubmods`
  (params (OwningWidget :type "Widget Object Reference"))
  (returns (Output1 :type "Array of /Game/Blueprints/BP_Submod_Model Object Reference"))
  (locals (Slots :type "Array of EImplantSlot Enum") (Output :type "Array of /Game/Blueprints/BP_Submod_Model Object Reference"))
  (bind _returnvalue (`Actor.GetComponentByClass` (`GameplayStatics.GetPlayerCharacter` (`local.__WorldContext`)) "/Script/TechBreach.ModulesComponent"))
  (`|ExecutionSequence`
    (:`then_0`
      (for _array_element (`ModulesComponent.InactiveSubmodules` _returnvalue)
        (bind _returnvalue_2 (`|GenericCreateObject` (`local.OwningWidget`) "/Game/Blueprints/BP_Submod_Model.BP_Submod_Model_C" _array_element 0 false))
        (`KismetArrayLibrary.Array_Add` (`local.Output`) _returnvalue_2)))
    (:`then_1`
      (for _array_element_2 (`local.Slots`)
        (bind (_value _returnvalue_3) (`BlueprintMapLibrary.Map_Find` (`ModulesComponent.ActiveImplants` _returnvalue) _array_element_2))
        (if _returnvalue_3
          (for (_array_element_3 _array_index) (`.InstalledSubmodules` (break `ImplantData` _value))
            (bind _returnvalue_4 (`|GenericCreateObject` (`local.OwningWidget`) "/Game/Blueprints/BP_Submod_Model.BP_Submod_Model_C" _array_element_3 _array_index true))
            (`KismetArrayLibrary.Array_Add` (`local.Output`) _returnvalue_4))))
      (return (`local.Output`)))))

(fn `GetPlayerActiveHudWidget`
  (returns (CommonActivatableWidget :type "CommonActivatableWidget Object Reference"))
  ;[1 1 1] horrifying, use interface later
  (bind _asbp_player_character (cast `/Game/Blueprints/Player/BP_PlayerCharacter` (`GameplayStatics.GetPlayerCharacter` (`local.__WorldContext`))))
  (if (`self.IsPlayerAlive` _asbp_player_character)
    (bind _widgetcanvas (`/Game/Blueprints/Player/BP_PlayerCharacter.WidgetCanvas` _asbp_player_character))
    (`/Engine/EditorBlueprintResources/StandardMacros.IsValid` _widgetcanvas
      (:`Is Valid`
        (bind _commonactivatablewidget (`/Game/Blueprints/UI/CommonUI/WBP_UserbaseCanvas.GetActiveWidget` _widgetcanvas))
        (return _commonactivatablewidget)))
    (else
      (`KismetSystemLibrary.PrintString` (`local.__WorldContext`) "GetPlayerActiveHudWidget: Player is dead"))))

(fn `GetPlayerMainCanvas`
  (returns (WidgetCanvas :type "/Game/Blueprints/UI/CommonUI/WBP_UserbaseCanvas Object Reference") (bExists :type Boolean))
  ;[1 1 1] horrifying, use interface later
  (bind _asbp_player_character (cast `/Game/Blueprints/Player/BP_PlayerCharacter` (`GameplayStatics.GetPlayerCharacter` (`local.__WorldContext`)))
    (:`then`
      (return (`/Game/Blueprints/Player/BP_PlayerCharacter.WidgetCanvas` _asbp_player_character) true))
    (:`CastFailed`
      (return null false))))

(fn `GetQuestsForMenu`
  (returns (Quests :type "Array of /Game/Blueprints/QuestSystem/F_QuestDetails Structure"))
  (bind _quests (`/Game/Blueprints/QuestSystem/AC_QuestLogComponent.GetVisibleAndCompletedQuests` (`Actor.GetComponentByClass` (`GameplayStatics.GetPlayerCharacter` (`local.__WorldContext`)) "/Game/Blueprints/QuestSystem/AC_QuestLogComponent.AC_QuestLogComponent_C")))
  (return _quests))

(fn `GetSubmodStatsFormatted`
  (params (SubmodData :type "SubmoduleData Structure"))
  (returns (SubmodStatsFormatted :type Text))
  (locals (Output :type Text) (AttributeTypes :type "Array of EAttributeType Enum"))
  (bind (_aoedata _weaponmesh _fireeffect _firesound _firemode _projectile _meshsocketname _spawnsocketname _weaponrelativelocation _weaponrelativerotation _weaponscale _damage _firerate _energyusage) (break `WeaponData` SubmodData_WeaponData))
  (bind _output (`local.Output`))
  (for _array_element (`local.AttributeTypes`)
    (bind _value (`BlueprintMapLibrary.Map_Find` SubmodData_AttributeCoefTerms _array_element))
    (if (!= _value 0.0)
      (if (`KismetTextLibrary.TextIsEmpty` (`local.Output`))
        (bind _returnvalue (`|GetEnumeratorNameAsString` _array_element))
        (bind _returnvalue_2 (`KismetTextLibrary.Conv_DoubleToText` _value "HalfToEven" true true 1 324 2 2))
        (set `local.Output` (`|FormatText` "{attribute}: {value}" _returnvalue _returnvalue_2))
        (else
          (set `local.Output` (`|FormatText` "{before} \n{attribute}: {value}" (`local.Output`) _returnvalue _returnvalue_2))))))
  (`|ExecutionSequence`
    (:`then_0`
      (if (!= _damage 0.0)
        (set `local.Output` (`|FormatText` "{before} \nDamage: {value}" _output (`KismetTextLibrary.Conv_DoubleToText` _damage "HalfToEven" true true 1 324 2 2)))
        (elif (!= (`.Damage` (break `DamageDataAoE` _aoedata)) 0.0)
          (set `local.Output` (`|FormatText` "{before} \nDamage: {value}" _output (`KismetTextLibrary.Conv_DoubleToText` (`.Damage` (break `DamageDataAoE` _aoedata)) "HalfToEven" true true 1 324 2 2))))))
    (:`then_1`
      (if (!= _firerate 0.0)
        (set `local.Output` (`|FormatText` "{before} \nFire rate (seconds): {value}" _output (`KismetTextLibrary.Conv_DoubleToText` _firerate "HalfToEven" true true 1 324 2 2)))))
    (:`then_2`
      (if (!= _energyusage 0.0)
        (set `local.Output` (`|FormatText` "{before} \nEnergy usage: {value}" _output (`KismetTextLibrary.Conv_DoubleToText` _energyusage "HalfToEven" true true 1 324 2 2)))))
    (:`then_3`
      (return (`local.Output`)))))

(fn `IsImplantSlotUsed`
  (params (ImplantSlot :type "EImplantSlot Enum" :default "Head1"))
  (returns (CurrentModule :type "ImplantData Structure") (bInUse :type Boolean))
  (bind (_value _returnvalue) (`BlueprintMapLibrary.Map_Find` (`ModulesComponent.ActiveImplants` (`Actor.GetComponentByClass` (`GameplayStatics.GetPlayerCharacter` (`local.__WorldContext`)) "/Script/TechBreach.ModulesComponent")) ImplantSlot))
  (return _value _returnvalue))

(fn `IsPlayerAlive`
  (returns (bIsAlive :type Boolean))
  (return (> (`StatsComponent.HealthCurrent` (`Actor.GetComponentByClass` (`GameplayStatics.GetPlayerCharacter` (`local.__WorldContext`)) "/Script/TechBreach.StatsComponent")) 0.0)))

(fn `LoadAudioSettings`
  (returns (bExists :type Boolean) (AudioSettings :type "Array of /Game/Blueprints/UI/F_AudioSetting Structure"))
  (locals (AudioSave :type String :default "save_audio_settings"))
  (bind _returnvalue (`GameplayStatics.DoesSaveGameExist` (`local.AudioSave`)))
  (if _returnvalue
    (bind _returnvalue_2 (`GameplayStatics.LoadGameFromSlot` (`local.AudioSave`)))
    (bind _asbp_save_game_audio_settings (cast `/Game/Blueprints/UI/BP_SaveGame_AudioSettings` _returnvalue_2)
      (:`then`
        (return true (`/Game/Blueprints/UI/BP_SaveGame_AudioSettings.AudioSettings` _asbp_save_game_audio_settings)))
      (:`CastFailed`
        _)))
  (return false))

(fn `LoadGameplaySettings`
  (returns (bExists :type Boolean) (GameplaySettings :type "Array of /Game/Blueprints/UI/F_GameplaySetting Structure"))
  (locals (GameplaySave :type String :default "save_gameplay_settings"))
  (bind _returnvalue (`GameplayStatics.DoesSaveGameExist` (`local.GameplaySave`)))
  (if _returnvalue
    (bind _returnvalue_2 (`GameplayStatics.LoadGameFromSlot` (`local.GameplaySave`)))
    (bind _asbp_save_game_gameplay_settings (cast `/Game/Blueprints/UI/BP_SaveGame_GameplaySettings` _returnvalue_2)
      (:`then`
        (return true (`/Game/Blueprints/UI/BP_SaveGame_GameplaySettings.GameplaySettings` _asbp_save_game_gameplay_settings)))
      (:`CastFailed`
        _)))
  (return false))

(fn `PushWidgetToMainCanvas`
  (params (ActivatableWidgetClass :type "CommonActivatableWidget Class Reference"))
  (bind (_widgetcanvas _bexists) (`self.GetPlayerMainCanvas` (`local.__WorldContext`)))
  (if _bexists
    (`/Game/Blueprints/UI/CommonUI/WBP_UserbaseCanvas.PushWidget` _widgetcanvas ActivatableWidgetClass)))

(fn `QuestUpdateModuleInstallation`
  (params (ImplantModuleId :type Name))
  (if (== ImplantModuleId "AL01")
    (`self.CompleteObjective` "Q_M_Test01_S02_O01" (`local.__WorldContext`))
    (bind _returnvalue (`GameplayStatics.GetActorOfClass` (`local.__WorldContext`) "/Game/Blueprints/Level/Scripting/BP_ImplantStatusManager_Base.BP_ImplantStatusManager_Base_C"))
    (`/Engine/EditorBlueprintResources/StandardMacros.IsValid` _returnvalue
      (:`Is Valid`
        (`/Game/Blueprints/Level/Scripting/BP_ImplantStatusManager_Base.ImplantInstalled` _returnvalue ImplantModuleId)))))

(fn `RemoveCenterContainerWidget`
  (bind _commonactivatablewidget (`self.GetPlayerActiveHudWidget` (`local.__WorldContext`)))
  (bind _aswbp_hud_base (cast `/Game/Blueprints/UI/HUD/WBP_HUD_Base` _commonactivatablewidget)
    (:`then`
      (bind _containercenter (`/Game/Blueprints/UI/HUD/WBP_HUD_Base.ContainerCenter` _aswbp_hud_base))
      (`/Engine/EditorBlueprintResources/StandardMacros.IsValid` _containercenter
        (:`Is Valid`
          (bind _commonactivatablewidget_2 (`/Game/Blueprints/UI/CommonUI/WBP_UserbaseCanvas.GetActiveWidget` _containercenter))
          (`/Game/Blueprints/UI/CommonUI/WBP_UserbaseCanvas.RemoveWidget` _containercenter _commonactivatablewidget_2))
        (:`Is Not Valid`
          (`KismetSystemLibrary.PrintString` (`local.__WorldContext`) "RemoveProgressBarWidget: Progress Bar Container not valid"))))
    (:`CastFailed`
      (`KismetSystemLibrary.PrintString` (`local.__WorldContext`) "RemoveProgressBarWidget: Cast to HUD Base failed"))))

(fn `RemoveImplantModule`
  (params (ImplantSlot :type "EImplantSlot Enum" :default "Head1"))
  (`ModulesComponent.RemoveImplant` (`Actor.GetComponentByClass` (`GameplayStatics.GetPlayerCharacter` (`local.__WorldContext`)) "/Script/TechBreach.ModulesComponent") ImplantSlot)
  (`GameplayStatics.PlaySound2D` (`local.__WorldContext`) "/Game/Audio/Misc/MS_Module_Install_End.MS_Module_Install_End" 1.0 1.0 0.0 null null))

(fn `RemoveMainCanvasWidget`
  (bind (_widgetcanvas _bexists) (`self.GetPlayerMainCanvas` (`local.__WorldContext`)))
  (if _bexists
    (bind _latestwidget (`/Game/Blueprints/UI/CommonUI/WBP_UserbaseCanvas.LatestWidget` _widgetcanvas))
    (`/Engine/EditorBlueprintResources/StandardMacros.IsValid` _latestwidget
      (:`Is Valid`
        (`/Game/Blueprints/UI/CommonUI/WBP_UserbaseCanvas.RemoveWidget` _widgetcanvas _latestwidget)))))

(fn `SaveAudioSettings`
  (params (AudioSettings :type "Array of /Game/Blueprints/UI/F_AudioSetting Structure"))
  (returns (ReturnValue :type Boolean))
  (locals (AudioSave :type String :default "save_audio_settings"))
  (bind _returnvalue (`GameplayStatics.CreateSaveGameObject` "/Game/Blueprints/UI/BP_SaveGame_AudioSettings.BP_SaveGame_AudioSettings_C"))
  (set `/Game/Blueprints/UI/BP_SaveGame_AudioSettings.AudioSettings` AudioSettings _returnvalue)
  (bind _returnvalue_2 (`GameplayStatics.SaveGameToSlot` _returnvalue (`local.AudioSave`)))
  (return _returnvalue_2))

(fn `SaveGameplaySettings`
  (params (GameplaySettings :type "Array of /Game/Blueprints/UI/F_GameplaySetting Structure"))
  (returns (ReturnValue :type Boolean))
  (locals (GameplaySave :type String :default "save_gameplay_settings"))
  (bind _returnvalue (`GameplayStatics.CreateSaveGameObject` "/Game/Blueprints/UI/BP_SaveGame_GameplaySettings.BP_SaveGame_GameplaySettings_C"))
  (set `/Game/Blueprints/UI/BP_SaveGame_GameplaySettings.GameplaySettings` GameplaySettings _returnvalue)
  (bind _returnvalue_2 (`GameplayStatics.SaveGameToSlot` _returnvalue (`local.GameplaySave`)))
  (return _returnvalue_2))

(fn `SetInputMode`
  (params (bSetToUI :type Boolean) (InWidgetToFocus :type "Widget Object Reference") (bShowMouse :type Boolean :default true))
  (bind _returnvalue (`GameplayStatics.GetPlayerController` (`local.__WorldContext`)))
  (if bSetToUI
    (`Controller.SetIgnoreMoveInput` _returnvalue true)
    (`WidgetBlueprintLibrary.SetInputMode_UIOnlyEx` _returnvalue InWidgetToFocus)
    (set `PlayerController.bShowMouseCursor` bShowMouse _returnvalue)
    (else
      (`WidgetBlueprintLibrary.SetInputMode_GameOnly` _returnvalue)
      (set `PlayerController.bShowMouseCursor` false _returnvalue)
      (`Controller.SetIgnoreMoveInput` _returnvalue false))))

(fn `ShowHint`
  (params (Text :type Text) (Duration :type "Float (double-precision)" :default 3.0) (bPlaySound :type Boolean :default true))
  (bind ___worldcontext (`local.__WorldContext`))
  (bind _commonactivatablewidget (`self.GetPlayerActiveHudWidget` ___worldcontext))
  (`/Engine/EditorBlueprintResources/StandardMacros.IsValid` _commonactivatablewidget
    (:`Is Valid`
      (bind _aswbp_hud_base (cast `/Game/Blueprints/UI/HUD/WBP_HUD_Base` _commonactivatablewidget))
      (`/Game/Blueprints/UI/HUD/WBP_HUD_Base.ShowHint` _aswbp_hud_base (`local.Text`) (`local.Duration`))
      (if bPlaySound
        (`GameplayStatics.PlaySound2D` ___worldcontext "/Game/Audio/UI/Waves/S_UI_Hint_01.S_UI_Hint_01" 1.0 1.0 0.0 null null)))))

(fn `ShowHudMessage`
  (params (SenderName :type String) (Message :type String) (SenderImage :type "Texture2D Object Reference") (bOverrideColor :type Boolean) (Color :type "LinearColor Structure") (Audio :type "SoundBase Object Reference") (TimeBeforeDisplay :type "Float (double-precision)" :default 1.0))
  (bind _asbp_player_character (cast `/Game/Blueprints/Player/BP_PlayerCharacter` (`GameplayStatics.GetPlayerCharacter` (`local.__WorldContext`))))
  (`/Game/Blueprints/UI/HUD/WBP_MessageContainer.DisplayMessage` (`/Game/Blueprints/Player/BP_PlayerCharacter.MessageWidget` _asbp_player_character) SenderName Message SenderImage bOverrideColor Color TimeBeforeDisplay)
  (`/Engine/EditorBlueprintResources/StandardMacros.IsValid` Audio
    (:`Is Valid`
      (`GameplayStatics.PlaySound2D` (`local.__WorldContext`) Audio 1.0 1.0 0.0 null null false))))

(fn `ShowHudMessageSubtitled`
  (params (SenderName :type String) (Message :type String) (SenderImage :type "Texture2D Object Reference") (bOverrideColor :type Boolean) (Color :type "LinearColor Structure") (Audio :type "SoundBase Object Reference") (TimeBeforeDisplay :type "Float (double-precision)" :default 1.0) (Subtitles :type "DataTable Object Reference"))
  (bind ___worldcontext (`local.__WorldContext`))
  (bind _returnvalue (`GameplayStatics.GetPlayerController` ___worldcontext))
  (bind _asbp_player_character (cast `/Game/Blueprints/Player/BP_PlayerCharacter` (`GameplayStatics.GetPlayerCharacter` ___worldcontext)))
  (bind _astech_game_instance (cast `TechGameInstance` (`GameplayStatics.GetGameInstance` ___worldcontext))
    (:`then`
      (bind (_gameplayoptions_healthcoefplayer _gameplayoptions_healthcoefenemy _gameplayoptions_mousesensitivity _gameplayoptions_mouseysign _gameplayoptions_showsubtitles) (break `GameplayOptions` (`TechGameInstance.GameplayOptions` _astech_game_instance)))
      (if _gameplayoptions_showsubtitles
        (`/Engine/EditorBlueprintResources/StandardMacros.IsValid` _returnvalue
          (:`Is Valid`
            (bind _asbp_tech_player_controller (cast `/Game/Blueprints/Player/BP_TechPlayerController` _returnvalue))
            (bind _returnvalue_2 (`|CreateWidget` "/Game/Blueprints/UI/Subtitles/WBP_Subtitles.WBP_Subtitles_C" _returnvalue (make `DataTableRowHandle` Subtitles "1")))
            (`UserWidget.AddToViewport` _returnvalue_2 0)
            (set `/Game/Blueprints/Player/BP_TechPlayerController.SubtitleWidget` _returnvalue_2 _asbp_tech_player_controller)))))
    (:`CastFailed`
      _))
  (`/Game/Blueprints/UI/HUD/WBP_MessageContainer.DisplayMessage` (`/Game/Blueprints/Player/BP_PlayerCharacter.MessageWidget` _asbp_player_character) SenderName Message SenderImage bOverrideColor Color TimeBeforeDisplay)
  (`/Engine/EditorBlueprintResources/StandardMacros.IsValid` Audio
    (:`Is Valid`
      (`GameplayStatics.PlaySound2D` (`local.__WorldContext`) Audio 1.0 1.0 0.0 null null false))))

(fn `ShowImplantInstallationMenu`
  (params (NewModule :type "ImplantData Structure") (CallingActor :type "Actor Object Reference"))
  (bind (_widgetcanvas _bexists) (`self.GetPlayerMainCanvas` (`local.__WorldContext`)))
  (if _bexists
    (`/Game/Blueprints/UI/CommonUI/WBP_UserbaseCanvas.PushWidget` _widgetcanvas "/Game/Blueprints/UI/HUD/WBP_InstallMenu_ImplantItem.WBP_InstallMenu_ImplantItem_C")
    (bind _commonactivatablewidget (`/Game/Blueprints/UI/CommonUI/WBP_UserbaseCanvas.GetActiveWidget` _widgetcanvas))
    (bind _aswbp_install_menu_implant_item (cast `/Game/Blueprints/UI/HUD/WBP_InstallMenu_ImplantItem` _commonactivatablewidget))
    (set `/Game/Blueprints/UI/HUD/WBP_InstallMenu_ImplantItem.NewModule` NewModule _aswbp_install_menu_implant_item)
    (set `/Game/Blueprints/UI/HUD/WBP_InstallMenu_ImplantItem.CallingActor` CallingActor _aswbp_install_menu_implant_item)
    (`/Game/Blueprints/UI/HUD/WBP_InstallMenu_ImplantItem.SetUp` _aswbp_install_menu_implant_item)))

(fn `ShowSubmodInstallationMenu`
  (params (NewSubmod :type "SubmoduleData Structure") (CallingActor :type "Actor Object Reference"))
  (bind (_widgetcanvas _bexists) (`self.GetPlayerMainCanvas` (`local.__WorldContext`)))
  (if _bexists
    (`/Game/Blueprints/UI/CommonUI/WBP_UserbaseCanvas.PushWidget` _widgetcanvas "/Game/Blueprints/UI/HUD/WBP_InstallMenu_SubmodItem.WBP_InstallMenu_SubmodItem_C")
    (bind _commonactivatablewidget (`/Game/Blueprints/UI/CommonUI/WBP_UserbaseCanvas.GetActiveWidget` _widgetcanvas))
    (bind _aswbp_install_menu_submod_item (cast `/Game/Blueprints/UI/HUD/WBP_InstallMenu_SubmodItem` _commonactivatablewidget))
    (set `/Game/Blueprints/UI/HUD/WBP_InstallMenu_SubmodItem.NewModule` (`local.NewSubmod`) _aswbp_install_menu_submod_item)
    (set `/Game/Blueprints/UI/HUD/WBP_InstallMenu_SubmodItem.CallingActor` (`local.CallingActor`) _aswbp_install_menu_submod_item)
    (`/Game/Blueprints/UI/HUD/WBP_InstallMenu_SubmodItem.SetUp` _aswbp_install_menu_submod_item)))

(fn `UnlockQuestStage`
  (params (StageId :type Name))
  (`/Game/Blueprints/QuestSystem/AC_QuestLogComponent.UnlockQuestStage` (`Actor.GetComponentByClass` (`GameplayStatics.GetPlayerCharacter` (`local.__WorldContext`)) "/Game/Blueprints/QuestSystem/AC_QuestLogComponent.AC_QuestLogComponent_C") StageId))

(fn `UpdateHudPlayerHealthAndEnergy`
  (params (EnergyPercentage :type "Float (double-precision)") (HealthPercentage :type "Float (double-precision)"))
  (bind _commonactivatablewidget (`self.GetPlayerActiveHudWidget` (`local.__WorldContext`)))
  ;[1 1 1] eww, use interfaces already
  (bind _aswbp_hud_base (cast `/Game/Blueprints/UI/HUD/WBP_HUD_Base` _commonactivatablewidget))
  (`/Game/Blueprints/UI/HUD/WBP_HUD_Base.Update Health and Energy` _aswbp_hud_base (`local.EnergyPercentage`) (`local.HealthPercentage`)))