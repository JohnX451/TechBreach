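; BP_Projectile_W01_A is a projectile actor that changes size with distance travelled and destroys itself at its maximum range.
; BeginPlay records the spawn location and the X component of the starting scale.
; Each Tick measures straight-line distance from the spawn point and remaps it to a uniform scale between the initial and final values.
; Once that distance reaches MaxTravelDistance, the actor is destroyed.
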(event `self.ReceiveBeginPlay`
  (bind _returnvalue_x (`KismetMathLibrary.BreakVector` (`self.GetActorScale3D`)))
  (set `self.InitialPosition` (`self.K2_GetActorLocation`))
  (set `self.InitialScaleFactor` _returnvalue_x))

(event `self.ReceiveTick`
  (params (DeltaSeconds :type "Float (single-precision)"))
  (bind _returnvalue (`KismetMathLibrary.Vector_Distance` (`self.InitialPosition`) (`self.K2_GetActorLocation`)))
  (if (< _returnvalue (`self.MaxTravelDistance`))
    (`self.SetActorScale3D` (`KismetMathLibrary.Conv_DoubleToVector` (`KismetMathLibrary.MapRangeClamped` _returnvalue 0.0 (`self.MaxTravelDistance`) (`self.InitialScaleFactor`) (`self.FinalScale`))))
    (else
      (`self.K2_DestroyActor`))))

(fn `UserConstructionScript`)