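; Cyborg operator enemy character with health handled by BPCyborgComponent, a weapon, voice barks and hit effects.
; Damage is reported to AI perception and can trigger pain cries, while strong hits at depleted health hide the struck bone with gore, silencing the voice on headshots.
; Death detaches controller and weapon, ragdolls the mesh and fires a quest interaction.
; Getters supply AI with roam, patrol, range and weak-spot data, alongside a gait-based speed setter.
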(event `Death`
  (params (DeathType :type Byte))
  (bind _mesh (`self.Mesh`))
  (bind _voice (`self.Voice`))
  (`self.DetachFromControllerPendingDestroy`)
  (`BaseWeaponComponent.DetachWeaponMesh` (`self.BP_Cyborg_Weapon_01`))
  (`PrimitiveComponent.SetCollisionEnabled` _mesh "QueryAndPhysics")
  (`PrimitiveComponent.SetSimulatePhysics` _mesh true)
  (`ActorComponent.K2_DestroyComponent` (`self.CapsuleComponent`))
  (`/Game/Blueprints/QuestSystem/AC_QuestActorComponent.QuestInteraction` (`self.BP_QuestActorComponent`))
  (`/Engine/EditorBlueprintResources/StandardMacros.IsValid` _voice
    (:`Is Valid`
      (`AudioComponent.SetSound` _voice "/Game/Audio/Voice/CyborgOperator/MS_Voice_Cyborg01_Death.MS_Voice_Cyborg01_Death")
      (`AudioComponent.Play` _voice 0.0)
      (`KismetSystemLibrary.Delay` 3.0)
      (`/Game/Blueprints/Components/AC_HitEffects.SpawnLiquidPoolOnFloor` (`self.AC_HitEffects`) (`SceneComponent.GetSocketLocation` (`self.Mesh`) "spine_04"))
      (`KismetSystemLibrary.Delay` 5.0)
      (`ActorComponent.SetComponentTickEnabled` (`self.Mesh`) false)
      (`self.SetActorTickEnabled` false))))

(event `self.ReceiveAnyDamage`
  (params (Damage :type "Float (single-precision)") (DamageType :type "DamageType Object Reference") (InstigatedBy :type "Controller Object Reference") (DamageCauser :type "Actor Object Reference"))
  (bind _voice (`self.Voice`))
  (`/Engine/EditorBlueprintResources/StandardMacros.IsValid` InstigatedBy
    (:`Is Valid`
      (`AISense_Damage.ReportDamageEvent` self InstigatedBy 0.0 (`self.K2_GetActorLocation` InstigatedBy)))
    (:`Is Not Valid`
      _))
  (bind _asdamage_type_extended (cast `DamageTypeExtended` DamageType))
  (if (and (`DamageTypeExtended.bCausePainReaction` _asdamage_type_extended) (`EnemyComponent.bIsAlive` (`self.BP_Cyborg_Component`)))
    (`/Engine/EditorBlueprintResources/StandardMacros.IsValid` _voice
      (:`Is Valid`
        (`AudioComponent.SetSound` _voice "/Game/Audio/Voice/CyborgOperator/MS_Voice_Cyborg01_Pain.MS_Voice_Cyborg01_Pain")
        (`AudioComponent.Play` _voice 0.0)))))

(event `self.SpawnHitEffect`
  (params (Damage :type "Float (single-precision)") (bIsWeakSpot :type Boolean) (HitLocation :type "Vector Structure") (HitNormal :type "Vector Structure") (HitBone :type Name))
  (`/Game/Blueprints/Components/AC_HitEffects.Spawn Impact Effect` (`self.AC_HitEffects`) 0 Damage bIsWeakSpot HitLocation HitNormal)
  (`self.HandleAppendageExplode` Damage HitBone HitLocation))

(event `/Game/Blueprints/Enemies/AI/BPI_EnemyAI.Vocalize`
  (params (SoundAsset :type "SoundBase Object Reference"))
  (bind _voice (`self.Voice`))
  (`/Engine/EditorBlueprintResources/StandardMacros.IsValid` SoundAsset
    (:`Is Valid`
      (`/Engine/EditorBlueprintResources/StandardMacros.IsValid` _voice
        (:`Is Valid`
          (`AudioComponent.SetSound` _voice SoundAsset)
          (`AudioComponent.Play` _voice 0.0))))))

(fn `GetFreeRoamData`
  (returns (FreeRoamOrigin :type "Vector Structure") (FreeRoamRadius :type Integer))
  (return (`self.FreeRoamOrigin`) (`self.FreeRoamRadius`)))

(fn `GetHitEffectInfo`
  (returns (ReturnValue :type "HitEffectData Structure"))
  (return (make `HitEffectData` 2.0 (`self.WeakSpots`))))

(fn `GetIdealRange`
  (returns (AttackRadius :type "Float (double-precision)") (DefendRadius :type "Float (double-precision)"))
  (return 200.0 1000.0))

(fn `GetPatrolRoute`
  (returns (PatrolRoute :type "/Game/Blueprints/Enemies/AI/BP_PatrolRoute Object Reference"))
  (return (`self.PatrolRoute`)))

(fn `HandleAppendageExplode`
  (params (Damage :type "Float (double-precision)") (BoneName :type Name) (HitLocation :type "Vector Structure"))
  (bind _voice (`self.Voice`))
  (if (and (< (`EnemyComponent.HealthCurrent` (`self.BP_Cyborg_Component`)) 1.0) (> Damage 15.0))
    (`SkinnedMeshComponent.HideBoneByName` (`self.Mesh`) BoneName "PBO_None")
    (`GameplayStatics.PlaySoundAtLocation` "/Game/Audio/Weapons/Impacts/MS_Hit_Flesh_Weakspot.MS_Hit_Flesh_Weakspot" HitLocation (struct) 1.0 1.0 0.0 null null null null)
    (`GameplayStatics.SpawnEmitterAtLocation` "/Game/ThirdParty/Realistic_Starter_VFX_Pack_Vol2/Particles/TechBreach/P_Blood_Splat_Spherical.P_Blood_Splat_Spherical" HitLocation)
    (if (== BoneName "head")
      (`/Engine/EditorBlueprintResources/StandardMacros.IsValid` _voice
        (:`Is Valid`
          (`AudioComponent.Stop` _voice)
          (`ActorComponent.K2_DestroyComponent` _voice))))))

(fn `IsAlive`
  (returns (bIsAlive :type Boolean))
  (return (`EnemyComponent.bIsAlive` (`self.BP_Cyborg_Component`))))

(fn `SetMovementSpeed`
  (params (Speed :type "/Game/Blueprints/Enemies/AI/Enums/E_MovementSpeed Enum" :default "NewEnumerator0"))
  (returns (SpeedValue :type "Float (double-precision)"))
  (bind _output_get (set `CharacterMovementComponent.MaxWalkSpeed` (select `/Game/Blueprints/Enemies/AI/Enums/E_MovementSpeed` Speed :`NewEnumerator1` 100.0 :`NewEnumerator2` 300.0 :`NewEnumerator3` 500.0 :!type "Float (single-precision)") (`self.CharacterMovement`)))
  (return _output_get))

(fn `UserConstructionScript`
  (set `/Game/Blueprints/Components/AC_Cyborg_Component.bShouldFreeRoam` (`self.bShouldFreeRoam`) (`self.BP_Cyborg_Component`))
  (if (== (`self.FreeRoamOrigin`) (0.0 0.0 0.0))
    (set `self.FreeRoamOrigin` (`self.K2_GetActorLocation`))))