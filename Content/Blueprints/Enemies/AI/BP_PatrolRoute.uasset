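; BP_PatrolRoute is an enemy AI patrol route actor that defines its waypoints as points on a spline component.
; IncrementPatrolRoute steps a patrol index along the spline by a direction value, flipping that direction at the last and first points for back-and-forth movement.
; GetSplinePointAsWorldPosition returns the current point's world location.
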(event `IncrementPatrolRoute`
  ;[1 1 1] Increment Patrol Point
  (bind _output_get (set `self.PatrolIndex` (+ (`self.PatrolIndex`) (`self.Direction`))))
  ;[1 1 1] Check if end of Patrol Route reached
  (if (== _output_get (- (`SplineComponent.GetNumberOfSplinePoints` (`self.PatrolRoute`)) 1))
    (set `self.Direction` -1)
    (else
      ;[1 1 1] Check if beginning of Patrol Route is reached
      (if (== (`self.PatrolIndex`) 0)
        (set `self.Direction` 1)))))

(fn `GetSplinePointAsWorldPosition`
  (returns (Location :type "Vector Structure"))
  (return (`SplineComponent.GetLocationAtSplinePoint` (`self.PatrolRoute`) (`self.PatrolIndex`) "World")))

(fn `UserConstructionScript`)